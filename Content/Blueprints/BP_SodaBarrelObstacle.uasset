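; BP_SodaBarrelObstacle is a barrel obstacle that gets knocked loose when a BP_BaseVehicle drives into it.
; The Box overlap turns on physics simulation for the SodaBarrel and, one second later, moves the actor to a fixed location below the world origin rather than destroying it.
; A DoOnce that resets after half a second throttles the barrel crash sound.
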(event `self.Box.OnComponentBeginOverlap`
  (params (OverlappedComponent :type "PrimitiveComponent Object Reference") (OtherActor :type "Actor Object Reference") (OtherComp :type "PrimitiveComponent Object Reference") (OtherBodyIndex :type Integer) (bFromSweep :type Boolean) (SweepResult :type "HitResult Structure (by ref)"))
  (cast `/Game/Blueprints/BP_BaseVehicle` OtherActor)
  (`PrimitiveComponent.SetSimulatePhysics` (`self.SodaBarrel`) true)
  (`|ExecutionSequence`
    (:`then_0`
      (`KismetSystemLibrary.Delay` 1.0)
      (`self.K2_SetActorLocation` (0.0 0.0 -1000.0)))
    (:`then_1`
      (`/Engine/EditorBlueprintResources/StandardMacros.DoOnce` false :!label _label
        (:`Completed`
          (`GameplayStatics.SpawnSoundAtLocation` "/Game/Sound/Obstacles/soda_barrels.soda_barrels" (0.0 0.0 0.0) (struct) 1.0 1.0 0.0 null null)
          (`KismetSystemLibrary.Delay` 0.5)
          (goto _label :!via `Reset`))))))

(fn `UserConstructionScript`
  (`parent.UserConstructionScript`))