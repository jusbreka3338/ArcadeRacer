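; Skateboard Blueprint that extends its parent's Tick with drift and rolling audio.
; Drifting spawns a drift sound at the DriftL component; ending the drift stops it and plays an end sound.
; CurrentSpeed crossing a threshold starts the rolling sound above it and stops it below.
; DoOnce gates that reset on opposite states keep the per-frame checks from retriggering sounds.
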(event `self.ReceiveTick`
  (params (DeltaSeconds :type "Float (single-precision)"))
  (bind _rev (`self.rev`))
  (bind _newvar_1 (`self.NewVar_1`))
  (bind _idle (`self.idle`))
  (`parent.ReceiveTick` DeltaSeconds)
  (`|ExecutionSequence`
    (:`then_0`
      (if (`self.Drifting`)
        (`|ExecutionSequence`
          (:`then_0`
            (`/Engine/EditorBlueprintResources/StandardMacros.DoOnce` false :!label _label
              (:`Completed`
                (bind _returnvalue (`GameplayStatics.SpawnSoundAtLocation` "/Game/Sound/Skateboardnoises/skateboard_drift_2.skateboard_drift_2" (`SceneComponent.K2_GetComponentLocation` (`self.Drift-L`)) (struct) 1.0 1.0 0.0 null null))
                (set `self.NewVar_1` _returnvalue))))
          (:`then_1`
            (goto _label_2 :!via `Reset`))
          (:`then_2`
            (`/Engine/EditorBlueprintResources/StandardMacros.DoOnce` false
              (:`Completed`
                (set `self.dont_spawnsound` true)))))
        (else
          (`|ExecutionSequence`
            (:`then_0`
              (`/Engine/EditorBlueprintResources/StandardMacros.IsValid` _newvar_1
                (:`Is Valid`
                  (if (`self.dont_spawnsound`)
                    (`AudioComponent.Stop` _newvar_1)
                    (`/Engine/EditorBlueprintResources/StandardMacros.DoOnce` false :!label _label_2
                      (:`Completed`
                        (`GameplayStatics.SpawnSoundAtLocation` "/Game/Sound/Skateboardnoises/skateboard_drift_end.skateboard_drift_end" (`SceneComponent.K2_GetComponentLocation` (`self.Drift-L`)) (struct) 1.0 1.0 0.0 null null)
                        (`KismetSystemLibrary.PrintString` "sound")))))))
            (:`then_1`
              (goto _label :!via `Reset`))))))
    (:`then_1`
      (if (< (`self.CurrentSpeed`) 150.0)
        (`|ExecutionSequence`
          (:`then_0`
            (`/Engine/EditorBlueprintResources/StandardMacros.DoOnce` false :!label _label_3
              (:`Completed`
                (`/Engine/EditorBlueprintResources/StandardMacros.IsValid` _rev
                  (:`Is Valid`
                    (`AudioComponent.Stop` _rev))))))
          (:`then_1`
            (goto _label_4 :!via `Reset`)))
        (else
          (`/Engine/EditorBlueprintResources/StandardMacros.DoOnce` false :!label _label_4
            (:`Completed`
              (bind _returnvalue_2 (`GameplayStatics.SpawnSoundAtLocation` "/Game/Sound/Skateboardnoises/skateboard_rolling.skateboard_rolling" (`SceneComponent.K2_GetComponentLocation` (`self.Drift-L`)) (struct) 1.0 1.0 0.0 null null))
              (set `self.rev` _returnvalue_2)
              (`/Engine/EditorBlueprintResources/StandardMacros.IsValid` _idle
                (:`Is Valid`
                  (`AudioComponent.Stop` _idle)
                  (goto _label_3 :!via `Reset`))))))))))

(fn `UserConstructionScript`
  (`parent.UserConstructionScript`))