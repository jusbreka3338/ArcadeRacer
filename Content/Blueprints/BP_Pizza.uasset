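; BP_Pizza is a spinning hazard that calls SpinOut on any BP_Scooter overlapping its Cube.
; Each Tick yaws the Cube by a fixed, frame-rate-dependent step and sets the actor's height above the last trace hit location.
; A short trace along FloorArrow, ignoring "HitSafe" actors, runs after the move, so height uses the previous frame's result, with no hit check.
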(event `self.ReceiveTick`
  (params (DeltaSeconds :type "Float (single-precision)"))
  (bind (_returnvalue_x _returnvalue_y) (`KismetMathLibrary.BreakVector` (`self.K2_GetActorLocation`)))
  (bind _cube (`self.Cube`))
  (bind _floorarrow (`self.FloorArrow`))
  (bind (_returnvalue_roll _returnvalue_pitch _returnvalue_yaw) (`KismetMathLibrary.BreakRotator` (`SceneComponent.K2_GetComponentRotation` _cube)))
  (bind _returnvalue (`SceneComponent.K2_GetComponentLocation` _floorarrow))
  (`|ExecutionSequence`
    (:`then_0`
      (`SceneComponent.K2_SetWorldRotation` _cube (`KismetMathLibrary.MakeRotator` _returnvalue_roll _returnvalue_pitch (+ _returnvalue_yaw 8.0)) false false)
      (`self.K2_SetActorLocation` (`KismetMathLibrary.MakeVector` _returnvalue_x _returnvalue_y (+ (.z (`.Location` (`GameplayStatics.BreakHitResult` (stale _outhit)))) 100.0))))
    (:`then_1`
      (bind _outactors (`GameplayStatics.GetAllActorsWithTag` "HitSafe"))
      (bind _outhit (`KismetSystemLibrary.LineTraceSingle` _returnvalue (+ _returnvalue (* (`KismetMathLibrary.GetForwardVector` (`SceneComponent.K2_GetComponentRotation` _floorarrow)) 150.0)) "TraceTypeQuery1" false _outactors)))))

(event `self.Cube.OnComponentBeginOverlap`
  (params (OverlappedComponent :type "PrimitiveComponent Object Reference") (OtherActor :type "Actor Object Reference") (OtherComp :type "PrimitiveComponent Object Reference") (OtherBodyIndex :type Integer) (bFromSweep :type Boolean) (SweepResult :type "HitResult Structure (by ref)"))
  (bind _asbp_scooter (cast `/Game/Blueprints/BP_Scooter` OtherActor))
  (`/Game/Blueprints/BP_Scooter.SpinOut` _asbp_scooter null))

(fn `UserConstructionScript`)