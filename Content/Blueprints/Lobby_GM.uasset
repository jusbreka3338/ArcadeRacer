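; Lobby game mode Blueprint that runs debug checks on the Lobby_Pawn actors at BeginPlay.
; CheckPlayer prints each pawn's controller name with a "Hi" suffix.
; After a short delay it calls a color-testing event, which is currently empty.
; Disconnected, never-run logic would give each pawn one of four player materials by matching its owner to the player controller index.
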(event `self.ReceiveBeginPlay`
  (`|ExecutionSequence`
    (:`then_0`
      (`self.CheckPlayer`))
    (:`then_3`
      (`KismetSystemLibrary.Delay` 0.2)
      (`self.Chang eColors testing`))))

(event `CheckPlayer`
  (bind _outactors (`GameplayStatics.GetAllActorsOfClass` "/Game/Blueprints/Lobby_Pawn.Lobby_Pawn_C"))
  (for _array_element _outactors
    (`KismetSystemLibrary.PrintString` (`KismetStringLibrary.Concat_StrStr` (`KismetSystemLibrary.GetDisplayName` (`Pawn.GetController` _array_element)) "Hi"))))

(event `Chang eColors testing`)

(fn `UserConstructionScript`)