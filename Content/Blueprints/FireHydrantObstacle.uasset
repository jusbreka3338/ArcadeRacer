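; Fire hydrant obstacle that starts shooting a water jet one second after a BP_Scooter overlaps its box, with nothing here turning it off.
; While active, Tick runs a debug-drawn line trace forward from an Arrow component.
; A scooter hit by the trace is pushed along the arrow by a fixed per-frame offset without sweeping.
; A DoOnce zeroes the scooter's CurrentSpeed on first contact and resets when the trace misses.
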(event `self.Box.OnComponentBeginOverlap`
  (params (OverlappedComponent :type "PrimitiveComponent Object Reference") (OtherActor :type "Actor Object Reference") (OtherComp :type "PrimitiveComponent Object Reference") (OtherBodyIndex :type Integer) (bFromSweep :type Boolean) (SweepResult :type "HitResult Structure (by ref)"))
  (cast `/Game/Blueprints/BP_Scooter` OtherActor)
  (`KismetSystemLibrary.Delay` 1.0)
  (set `self.WaterShoot` true))

(event `self.ReceiveTick`
  (params (DeltaSeconds :type "Float (single-precision)"))
  (bind _arrow (`self.Arrow`))
  (bind _returnvalue (`SceneComponent.K2_GetComponentLocation` _arrow))
  (if (`self.WaterShoot`)
    (bind _outhit (`KismetSystemLibrary.LineTraceSingle` :`Start` _returnvalue :`End` (+ _returnvalue (* (`SceneComponent.GetForwardVector` _arrow) 750.0)) :`TraceChannel` "TraceTypeQuery1" :`DrawDebugType` "ForDuration" :`DrawTime` 0.1))
    (bind _asbp_scooter (cast `/Game/Blueprints/BP_Scooter` (`.HitActor` (`GameplayStatics.BreakHitResult` _outhit)))
      (:`then`
        (`self.K2_AddActorWorldOffset` _asbp_scooter (* (`SceneComponent.GetForwardVector` (`self.Arrow`)) 20.0) false false)
        (`/Engine/EditorBlueprintResources/StandardMacros.DoOnce` false :!label _label
          (:`Completed`
            (set `/Game/Blueprints/BP_Scooter.CurrentSpeed` 0.0 _asbp_scooter))))
      (:`CastFailed`
        (goto _label :!via `Reset`)))))

(fn `UserConstructionScript`)