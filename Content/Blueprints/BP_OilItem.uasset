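; Oil item actor that places itself on a surface when it spawns.
; BeginPlay line-traces along its Arrow, ignoring actors tagged HitSafe, and moves the actor to the impact point, sunk slightly along Z.
; The hit result is not checked before the move.
; A Safety flag is held true for a short delay after placement, then cleared; nothing in this graph reads it.
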(event `self.ReceiveBeginPlay`
  (bind _arrow (`self.Arrow`))
  (bind _returnvalue (`SceneComponent.K2_GetComponentLocation` _arrow))
  (`parent.ReceiveBeginPlay`)
  (set `self.Safety` true)
  (bind _outactors (`GameplayStatics.GetAllActorsWithTag` "HitSafe"))
  (bind _outhit (`KismetSystemLibrary.LineTraceSingle` _returnvalue (+ _returnvalue (* (`KismetMathLibrary.GetForwardVector` (`SceneComponent.K2_GetComponentRotation` _arrow)) 1500.0)) "TraceTypeQuery1" false _outactors))
  (`self.K2_SetActorLocation` (+ (`.ImpactPoint` (`GameplayStatics.BreakHitResult` _outhit)) (0.0 0.0 -20.0)))
  (`KismetSystemLibrary.Delay` 0.5)
  (set `self.Safety` false))

(fn `UserConstructionScript`
  (`parent.UserConstructionScript`))