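; Player controller that lets a player toggle joining and leaving the game with the ConnectPlayer input action.
; After a short delay, a FlipFlop alternates between asking ConnectPlayer_GM to spawn a character for this controller and to despawn it.
; The controller holds no other active logic, as a debug print of the controlled pawn's name is left disconnected from any event.
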(event `InputAction|ConnectPlayer`
  (params (Key :type "Key Structure"))
  (:`Pressed`
    (`KismetSystemLibrary.Delay` 0.2)
    (`/Engine/EditorBlueprintResources/StandardMacros.FlipFlop`
      (:`A`
        (bind _asconnect_player_gm (cast `/Game/Blueprints/ConnectPlayer_GM` (`GameplayStatics.GetGameMode`)))
        (`/Game/Blueprints/ConnectPlayer_GM.SpawnCharacter` _asconnect_player_gm self)
        (`KismetSystemLibrary.Delay` 0.2))
      (:`B`
        (bind _asconnect_player_gm_2 (cast `/Game/Blueprints/ConnectPlayer_GM` (`GameplayStatics.GetGameMode`)))
        (`/Game/Blueprints/ConnectPlayer_GM.DespawnPlayer` _asconnect_player_gm_2 self)
        (`KismetSystemLibrary.Delay` 0.2)))))

(fn `UserConstructionScript`)