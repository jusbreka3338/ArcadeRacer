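; BP_TrashBag is a physics-launched hazard that spins out scooters that touch it.
; On BeginPlay it finds the first BP_Scooter and applies a mass-independent impulse to its mesh, upward and along that scooter's forward axis, scaled by its current speed.
; A short delay then clears the Safe flag, after which any scooter overlapping the mesh gets SpinOut called.
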(event `self.ReceiveBeginPlay`
  (bind _outactors (`GameplayStatics.GetAllActorsOfClass` "/Game/Blueprints/BP_Scooter.BP_Scooter_C"))
  (bind _output_get (set `self.ScooterRef` (`|GetArrayItem` _outactors)))
  (`PrimitiveComponent.AddImpulse` (`self.StaticMesh`) (`KismetMathLibrary.TransformDirection` (`self.GetTransform` _output_get) (`KismetMathLibrary.MakeVector` (* (`/Game/Blueprints/BP_Scooter.CurrentSpeed` _output_get) 1.5) 0.0 1000.0)) "None" true)
  (`KismetSystemLibrary.Delay` 0.3)
  (set `self.Safe` false))

(event `self.StaticMesh.OnComponentBeginOverlap`
  (params (OverlappedComponent :type "PrimitiveComponent Object Reference") (OtherActor :type "Actor Object Reference") (OtherComp :type "PrimitiveComponent Object Reference") (OtherBodyIndex :type Integer) (bFromSweep :type Boolean) (SweepResult :type "HitResult Structure (by ref)"))
  (bind _asbp_scooter (cast `/Game/Blueprints/BP_Scooter` OtherActor))
  (if (not (`self.Safe`))
    (`/Game/Blueprints/BP_Scooter.SpinOut` _asbp_scooter null)))

(fn `UserConstructionScript`)