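; Lobby player controller that handles character selection for four slots, storing each chosen class in the Arcade_GI game instance.
; Each ChangeCharacter event destroys the controlled pawn, spawns the given class at its transform, possesses it and saves the choice.
; Matching SetCharacterClass events only save the choice.
; BeginPlay calls an empty CreatMenus event, as the WGT_Lobby widget creation logic is disconnected and never runs.
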(event `self.ReceiveBeginPlay`
  (`self.CreatMenus`))

(event `CreatMenus`)

(event `ChangeCharacter`
  (params (CharRowName :type "/Game/Blueprints/BP_BaseVehicle Class Reference"))
  (bind _returnvalue (`self.K2_GetPawn`))
  (set `self.SpawnTransform` (`self.GetTransform` _returnvalue))
  (`self.K2_DestroyActor` _returnvalue)
  (bind _returnvalue_2 (`|SpawnActorFromClass` CharRowName (`self.SpawnTransform`) "Undefined" "MultiplyWithRoot" null null))
  (`self.Possess` _returnvalue_2)
  (bind _asarcade_gi (cast `/Game/Blueprints/Arcade_GI` (`GameplayStatics.GetGameInstance`)))
  (set `/Game/Blueprints/Arcade_GI.ChosenClass` CharRowName _asarcade_gi))

(event `SetCharacterClass`
  (params (ChosenClass :type "/Game/Blueprints/BP_BaseVehicle Class Reference"))
  (bind _asarcade_gi (cast `/Game/Blueprints/Arcade_GI` (`GameplayStatics.GetGameInstance`)))
  (set `/Game/Blueprints/Arcade_GI.ChosenClass` ChosenClass _asarcade_gi))

(event `ChangeCharacter2`
  (params (CharRowName2 :type "/Game/Blueprints/BP_BaseVehicle Class Reference"))
  (bind _returnvalue (`self.K2_GetPawn`))
  (set `self.SpawnTransform2` (`self.GetTransform` _returnvalue))
  (`self.K2_DestroyActor` _returnvalue)
  (bind _returnvalue_2 (`|SpawnActorFromClass` CharRowName2 (`self.SpawnTransform2`) "Undefined" "MultiplyWithRoot" null null))
  (`self.Possess` _returnvalue_2)
  (bind _asarcade_gi (cast `/Game/Blueprints/Arcade_GI` (`GameplayStatics.GetGameInstance`)))
  (set `/Game/Blueprints/Arcade_GI.ChosenClass2` CharRowName2 _asarcade_gi))

(event `SetCharacterClass2`
  (params (ChosenClass2 :type "/Game/Blueprints/BP_BaseVehicle Class Reference"))
  (bind _asarcade_gi (cast `/Game/Blueprints/Arcade_GI` (`GameplayStatics.GetGameInstance`)))
  (set `/Game/Blueprints/Arcade_GI.ChosenClass2` ChosenClass2 _asarcade_gi))

(event `ChangeCharacter3`
  (params (CharRowName3 :type "/Game/Blueprints/BP_BaseVehicle Class Reference"))
  (bind _returnvalue (`self.K2_GetPawn`))
  (set `self.SpawnTransform3` (`self.GetTransform` _returnvalue))
  (`self.K2_DestroyActor` _returnvalue)
  (bind _returnvalue_2 (`|SpawnActorFromClass` CharRowName3 (`self.SpawnTransform3`) "Undefined" "MultiplyWithRoot" null null))
  (`self.Possess` _returnvalue_2)
  (bind _asarcade_gi (cast `/Game/Blueprints/Arcade_GI` (`GameplayStatics.GetGameInstance`)))
  (set `/Game/Blueprints/Arcade_GI.ChosenClass3` CharRowName3 _asarcade_gi))

(event `SetCharacterClass3`
  (params (ChosenClass3 :type "/Game/Blueprints/BP_BaseVehicle Class Reference"))
  (bind _asarcade_gi (cast `/Game/Blueprints/Arcade_GI` (`GameplayStatics.GetGameInstance`)))
  (set `/Game/Blueprints/Arcade_GI.ChosenClass3` ChosenClass3 _asarcade_gi))

(event `ChangeCharacter4`
  (params (CharRowName4 :type "/Game/Blueprints/BP_BaseVehicle Class Reference"))
  (bind _returnvalue (`self.K2_GetPawn`))
  (set `self.SpawnTransform4` (`self.GetTransform` _returnvalue))
  (`self.K2_DestroyActor` _returnvalue)
  (bind _returnvalue_2 (`|SpawnActorFromClass` CharRowName4 (`self.SpawnTransform4`) "Undefined" "MultiplyWithRoot" null null))
  (`self.Possess` _returnvalue_2)
  (bind _asarcade_gi (cast `/Game/Blueprints/Arcade_GI` (`GameplayStatics.GetGameInstance`)))
  (set `/Game/Blueprints/Arcade_GI.ChosenClass4` CharRowName4 _asarcade_gi))

(event `SetCharacterClass4`
  (params (ChosenClass4 :type "/Game/Blueprints/BP_BaseVehicle Class Reference"))
  (bind _asarcade_gi (cast `/Game/Blueprints/Arcade_GI` (`GameplayStatics.GetGameInstance`)))
  (set `/Game/Blueprints/Arcade_GI.ChosenClass4` ChosenClass4 _asarcade_gi))

(fn `UserConstructionScript`)