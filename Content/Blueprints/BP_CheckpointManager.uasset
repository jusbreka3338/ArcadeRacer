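; Checkpoint manager for an arcade lap mode that tracks checkpoint hits and laps through Arcade_GM.
; On BeginPlay it binds each checkpoint's hit event, which advances the required index and updates progress text.
; Reaching the needed count increments laps and schedules a delayed reset, applied only if LapComplete is set.
; NEEDEDCHECKPOINT shows and enables query collision only on checkpoints matching the required index; here only the reset calls it.
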(event `NEEDED CHECKPOINT`
  (for _array_element (`self.Checkpoints`)
    (if (== (`/Game/Blueprints/Arcade_GM.CheckpointRequired` (stale `self.ReceiveBeginPlay` _asarcade_gm)) (`/Game/Blueprints/BP_CheckPoint.Checkpoint wanted` _array_element))
      (`PrimitiveComponent.SetCollisionEnabled` (`/Game/Blueprints/BP_CheckPoint.Cylinder` _array_element) "QueryOnly")
      (`self.SetActorHiddenInGame` _array_element false)
      (else
        (`PrimitiveComponent.SetCollisionEnabled` (`/Game/Blueprints/BP_CheckPoint.Cylinder` _array_element) "NoCollision")
        (`self.SetActorHiddenInGame` _array_element true)))))

(event `self.ReceiveBeginPlay`
  (bind _checkpoints (`self.Checkpoints`))
  (`KismetSystemLibrary.DelayUntilNextTick`)
  (`|ExecutionSequence`
    (:`then_0`
      (bind _asarcade_gm (cast `/Game/Blueprints/Arcade_GM` (`GameplayStatics.GetGameMode`)))
      (set `self.As Arcade GM` _asarcade_gm)
      (set `self.Checkpoint Required` (`KismetArrayLibrary.Array_Length` _checkpoints))
      (for _array_element _checkpoints
        (add `/Game/Blueprints/BP_CheckPoint.Checkpoint Hit` _array_element (delegate `CheckpointHit`))
        (set `/Game/Blueprints/Arcade_GM.CheckpointText` (`self.CheckpointsToText` (`self.#OfCheckpoints Needed`)) (`self.As Arcade GM`))))))

(event `CheckpointHit`
  (bind _as_arcade_gm (`self.As Arcade GM`))
  (bind _checkpointcount (`self.CheckpointCount`))
  (bind __ofcheckpoints_needed (`self.#OfCheckpoints Needed`))
  (bind _as_arcade_gm_2 (`self.As Arcade GM`))
  (`|ExecutionSequence`
    (:`then_0`
      (bind _result (`/Engine/EditorBlueprintResources/StandardMacros.IncrementInt` _checkpointcount)
        (:`  `
          (set `/Game/Blueprints/Arcade_GM.CheckpointText` (`self.CheckpointsToText` __ofcheckpoints_needed _result) (`self.As Arcade GM`))
          (if (== __ofcheckpoints_needed _checkpointcount)
            (`KismetSystemLibrary.K2_SetTimerDelegate` (delegate `ResetCheckpoints`) 1.0)
            (`/Engine/EditorBlueprintResources/StandardMacros.IncrementInt` (`/Game/Blueprints/Arcade_GM.LapsCompleted` _as_arcade_gm)
              (:`  `
                (`/Game/Blueprints/Arcade_GM.Update laps` _as_arcade_gm)))))))
    (:`then_1`
      (bind _result_2 (`/Engine/EditorBlueprintResources/StandardMacros.IncrementInt` (`/Game/Blueprints/Arcade_GM.CheckpointRequired` _as_arcade_gm_2))
        (:`  `
          (set `/Game/Blueprints/Arcade_GM.CheckpointRequired` _result_2 _as_arcade_gm_2))))))

(event `self.ReceiveTick`
  (params (DeltaSeconds :type "Float (single-precision)")))

(event `ResetCheckpoints`
  (bind _as_arcade_gm (`self.As Arcade GM`))
  (if (`/Game/Blueprints/Arcade_GM.LapComplete?` _as_arcade_gm)
    (set `/Game/Blueprints/Arcade_GM.LapComplete?` false _as_arcade_gm)
    (set `/Game/Blueprints/Arcade_GM.CheckpointRequired` 0 (`self.As Arcade GM`))
    (bind _output_get (set `self.CheckpointCount` 0))
    (set `/Game/Blueprints/Arcade_GM.CheckpointText` (`self.CheckpointsToText` (`self.#OfCheckpoints Needed`) _output_get) (`self.As Arcade GM`))
    (`self.NEEDED CHECKPOINT`)))

(fn `UserConstructionScript`)