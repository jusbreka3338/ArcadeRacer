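; BP_SkidMark is a skid mark actor that snaps itself to the height of the surface it finds when spawned.
; On BeginPlay it line traces along its Arrow component's forward vector on the Visibility channel, ignoring every BP_BaseVehicle actor.
; It keeps its X and Y and sets Z slightly below the impact point, without checking whether the trace hit.
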(event `self.ReceiveBeginPlay`
  (bind (_returnvalue_x _returnvalue_y) (`KismetMathLibrary.BreakVector` (`self.K2_GetActorLocation`)))
  (bind _arrow (`self.Arrow`))
  (bind _returnvalue (`SceneComponent.K2_GetComponentLocation` _arrow))
  (bind _outactors (`GameplayStatics.GetAllActorsOfClass` "/Game/Blueprints/BP_BaseVehicle.BP_BaseVehicle_C"))
  (bind _outhit (`KismetSystemLibrary.LineTraceSingle` _returnvalue (+ _returnvalue (* (`KismetMathLibrary.GetForwardVector` (`SceneComponent.K2_GetComponentRotation` _arrow)) 1500.0)) "TraceTypeQuery1" false _outactors))
  (`self.K2_SetActorLocation` (`KismetMathLibrary.MakeVector` _returnvalue_x _returnvalue_y (+ (.z (`.ImpactPoint` (`GameplayStatics.BreakHitResult` _outhit))) -17.0))))

(fn `UserConstructionScript`)