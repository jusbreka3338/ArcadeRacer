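; Trash can obstacle that reacts when the player's scooter runs into it.
; A box overlap with BP_Scooter switches on physics simulation for the can and lid meshes so they get knocked loose.
; One second later it moves the actor far below the level instead of destroying it.
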(event `self.Box.OnComponentBeginOverlap`
  (params (OverlappedComponent :type "PrimitiveComponent Object Reference") (OtherActor :type "Actor Object Reference") (OtherComp :type "PrimitiveComponent Object Reference") (OtherBodyIndex :type Integer) (bFromSweep :type Boolean) (SweepResult :type "HitResult Structure (by ref)"))
  (cast `/Game/Blueprints/BP_Scooter` OtherActor)
  (`PrimitiveComponent.SetSimulatePhysics` (`self.TrashCanMesh`) true)
  (`PrimitiveComponent.SetSimulatePhysics` (`self.LidMesh`) true)
  (`KismetSystemLibrary.Delay` 1.0)
  (`self.K2_SetActorLocation` (0.0 0.0 -1000.0)))

(fn `UserConstructionScript`
  (`parent.UserConstructionScript`))