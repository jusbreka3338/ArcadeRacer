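; Hanging light obstacle that sways on a cable and falls after being hit twice by BP_Scooter.
; A runtime-added static mesh carries the point light and follows the cable's first particle each Tick.
; A looping LightSway timeline drives cable force, and scooter overlaps briefly set it from the scooter's speed.
; The second hit deactivates Niagara and sets Fall, switching the mesh to physics simulation.
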(event `self.ReceiveBeginPlay`
  (bind _pointlight (`self.PointLight`))
  (bind _returnvalue (`AddComponent|NODE_AddStaticMeshComponent-0` :`bManualAttachment` true :`RelativeTransform` (`KismetMathLibrary.MakeTransform` (`|GetArrayItem` (`CableComponent.GetCableParticleLocations` (`self.Cable`))))))
  (`SceneComponent.K2_AttachToComponent` _pointlight _returnvalue "None" "KeepRelative" "KeepRelative" "KeepRelative" true)
  (`SceneComponent.K2_SetWorldLocation` _pointlight (`SceneComponent.K2_GetComponentLocation` _returnvalue) false false)
  (bind (_direction _newtrack_0) (`Timeline|LightSway` :!via `PlayFromStart` :!label _label)
    (:`Update`
      (bind _returnvalue_2 (* _newtrack_0 50.0))
      (set `CableComponent.CableForce` (`KismetMathLibrary.MakeVector` _returnvalue_2 (* _returnvalue_2 0.7)) (`self.Cable`)))
    (:`Finished`
      (`KismetSystemLibrary.Delay` 0.1)
      (goto _label :!via `PlayFromStart`))))

(event `self.ReceiveTick`
  (params (DeltaSeconds :type "Float (single-precision)"))
  (if (`self.Fall`)
    (`PrimitiveComponent.SetSimulatePhysics` (stale `self.ReceiveBeginPlay` _returnvalue) true)
    (else
      (`SceneComponent.K2_SetWorldLocation` (stale `self.ReceiveBeginPlay` _returnvalue) (`|GetArrayItem` (`CableComponent.GetCableParticleLocations` (`self.Cable`))) false false))))

(event `self.Box.OnComponentBeginOverlap`
  (params (OverlappedComponent :type "PrimitiveComponent Object Reference") (OtherActor :type "Actor Object Reference") (OtherComp :type "PrimitiveComponent Object Reference") (OtherBodyIndex :type Integer) (bFromSweep :type Boolean) (SweepResult :type "HitResult Structure (by ref)"))
  (bind _cable (`self.Cable`))
  (bind _asbp_scooter (cast `/Game/Blueprints/BP_Scooter` OtherActor))
  (`/Engine/EditorBlueprintResources/StandardMacros.DoOnce` false :!label _label_2
    (:`Completed`
      (`|ExecutionSequence`
        (:`then_0`
          (set `self.HitTimes` (+ (`self.HitTimes`) 1))
          (bind _currentspeed (`/Game/Blueprints/BP_Scooter.CurrentSpeed` _asbp_scooter))
          (set `CableComponent.CableForce` (`KismetMathLibrary.MakeVector` _currentspeed _currentspeed) _cable)
          (`KismetSystemLibrary.Delay` 0.2)
          (set `CableComponent.CableForce` (0.0 0.0 0.0) _cable)
          (if (> (`self.HitTimes`) 1)
            (`KismetSystemLibrary.PrintString` "fall")
            (set `self.Fall` true)
            (`ActorComponent.Deactivate` (`self.Niagara`))))))))

(event `self.Box.OnComponentEndOverlap`
  (params (OverlappedComponent :type "PrimitiveComponent Object Reference") (OtherActor :type "Actor Object Reference") (OtherComp :type "PrimitiveComponent Object Reference") (OtherBodyIndex :type Integer))
  (cast `/Game/Blueprints/BP_Scooter` OtherActor)
  (goto _label_2 :!via `Reset`))

(fn `UserConstructionScript`)