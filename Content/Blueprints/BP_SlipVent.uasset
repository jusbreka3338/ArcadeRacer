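; BP_SlipVent is a vent hazard or pickup that boosts a vehicle's slipstream bar.
; A self-repeating random delay flip-flops the vent and its Niagara particles on and off.
; Overlapping while active fires a DoOnce, re-armed on each turn-on, which shuts the vent off.
; Unless the vehicle is Dreaming, a timeline then adds to its stored bar value and updates the main HUD widget, clamping only the displayed value.
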(event `TurnOn`
  (`ActorComponent.Activate` (`self.NS_HueShiftStencilParticleStationary`) false)
  (set `self.SlipOn` true)
  (goto _label :!via `Reset`))

(event `TurnOff`
  (`ActorComponent.Deactivate` (`self.NS_HueShiftStencilParticleStationary`))
  (set `self.SlipOn` false))

(event `Countdown`
  (`KismetSystemLibrary.Delay` (`KismetMathLibrary.RandomFloatInRange` 5.0 10.0))
  (`/Engine/EditorBlueprintResources/StandardMacros.FlipFlop`
    (:`A`
      (`self.TurnOn`))
    (:`B`
      (`self.TurnOff`)))
  (`self.Countdown`))

(event `self.ReceiveBeginPlay`
  (`|ExecutionSequence`
    (:`then_0`
      (bind _outactors (`GameplayStatics.GetAllActorsOfClass` "/Game/Blueprints/BP_BaseVehicle.BP_BaseVehicle_C"))
      (set `self.BaseVehicle` (`|GetArrayItem` _outactors)))
    (:`then_1`
      (bind _foundwidgets (`WidgetBlueprintLibrary.GetAllWidgetsOfClass` "/Game/A_UI/WGT_Main.WGT_Main_C"))
      (set `self.Main WGTRef` (`|GetArrayItem` _foundwidgets)))
    (:`then_2`
      (`self.Countdown`))))

(event `self.Box.OnComponentBeginOverlap`
  (params (OverlappedComponent :type "PrimitiveComponent Object Reference") (OtherActor :type "Actor Object Reference") (OtherComp :type "PrimitiveComponent Object Reference") (OtherBodyIndex :type Integer) (bFromSweep :type Boolean) (SweepResult :type "HitResult Structure (by ref)"))
  (bind _asbp_base_vehicle (cast `/Game/Blueprints/BP_BaseVehicle` OtherActor))
  (if (`self.SlipOn`)
    (`/Engine/EditorBlueprintResources/StandardMacros.DoOnce` false :!label _label
      (:`Completed`
        (bind _output_get (set `self.StoredSlipBar` (`/Game/Blueprints/BP_BaseVehicle.Slipstreambar` _asbp_base_vehicle)))
        (`self.TurnOff`)
        (if (not (`/Game/Blueprints/BP_BaseVehicle.Dreaming` _asbp_base_vehicle))
          (bind (_direction _addamount) (`Timeline|SlipStreamFill` :!via `PlayFromStart`)
            (:`Update`
              (bind _output_get_2 (set `/Game/Blueprints/BP_BaseVehicle.Slipstreambar` (+ _output_get _addamount) _asbp_base_vehicle))
              (`/Game/A_UI/WGT_Main.Set SlipStreamBar` (`self.Main WGTRef`) (`KismetMathLibrary.FClamp` _output_get_2)))))))))

(fn `UserConstructionScript`)