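; BP_TrashBagBurst is a thrown trash bag hazard that spins out vehicles it touches.
; On BeginPlay it launches its mesh using the first BP_BaseVehicle found, with an impulse in that vehicle's local space scaled by speed, plus upward lift.
; A short delay clears the Safe flag, after which overlapping vehicles call SpinOut.
; Overlaps with mesh, spline or landscape spline types only print debug messages.
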(event `self.ReceiveBeginPlay`
  (bind _outactors (`GameplayStatics.GetAllActorsOfClass` "/Game/Blueprints/BP_BaseVehicle.BP_BaseVehicle_C"))
  (bind _output_get (set `self.ScooterRef` (`|GetArrayItem` _outactors)))
  (`PrimitiveComponent.AddImpulse` (`self.StaticMesh`) (`KismetMathLibrary.TransformDirection` (`self.GetTransform` _output_get) (`KismetMathLibrary.MakeVector` (* (`/Game/Blueprints/BP_BaseVehicle.CurrentSpeed` _output_get) (`self.ThrowDistance`)) 0.0 1000.0)) "None" true)
  (`KismetSystemLibrary.Delay` 0.3)
  (set `self.Safe` false))

(event `self.StaticMesh.OnComponentBeginOverlap`
  (params (OverlappedComponent :type "PrimitiveComponent Object Reference") (OtherActor :type "Actor Object Reference") (OtherComp :type "PrimitiveComponent Object Reference") (OtherBodyIndex :type Integer) (bFromSweep :type Boolean) (SweepResult :type "HitResult Structure (by ref)"))
  (`|ExecutionSequence`
    (:`then_0`
      (bind _asbp_base_vehicle (cast `/Game/Blueprints/BP_BaseVehicle` OtherActor))
      (if (not (`self.Safe`))
        (`/Game/Blueprints/BP_BaseVehicle.SpinOut` _asbp_base_vehicle null)))
    (:`then_1`
      (cast `SplineMeshComponent` OtherComp)
      (`KismetSystemLibrary.PrintString` "Hello" true true (struct :`R` 1.0 :`G` 0.044271 :`B` 0.233183 :`A` 1.0) :!label _label))
    (:`then_2`
      (cast `MeshComponent` OtherComp)
      (goto _label))
    (:`then_3`
      (cast `SplineComponent` OtherComp)
      (goto _label))
    (:`then_4`
      (cast `LandscapeSplinesComponent` OtherComp)
      (goto _label))
    (:`then_5`
      (cast `LandscapeSplineActor` OtherActor)
      (goto _label))))

(fn `UserConstructionScript`)