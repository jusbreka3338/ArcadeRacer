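; PauseMenuTestPawn is a test pawn that toggles the pause menu widget on the PauseMenu input.
; It reads IsInPauseMenu from the cached Arcade_GI to either create WGT_PauseMenu or remove it, clear the flag and restore game-only input.
; It never sets that flag true itself.
; A DoOnce with a short delayed reset debounces presses, and thumbstick-style mouse-movement code is left unconnected.
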(event `self.ReceiveBeginPlay`
  (bind _asarcade_gi (cast `/Game/Blueprints/Arcade_GI` (`GameplayStatics.GetGameInstance`)))
  (set `self.Arcade Game Instance` _asarcade_gi))

(event `InputAxis|NINputAxisTHUMBY`
  (params (AxisValue :type "Float (single-precision)")))

(event `InputAction|PauseMenu`
  (params (Key :type "Key Structure"))
  (bind _arcade_game_instance (`self.Arcade Game Instance`))
  (:`Pressed`
    (`/Engine/EditorBlueprintResources/StandardMacros.DoOnce` false :!label _label
      (:`Completed`
        (`|ExecutionSequence`
          (:`then_0`
            (if (`/Game/Blueprints/Arcade_GI.IsInPauseMenu?` _arcade_game_instance)
              (set `/Game/Blueprints/Arcade_GI.IsInPauseMenu?` false _arcade_game_instance)
              (`WidgetBlueprintLibrary.SetInputMode_GameOnly` null)
              (set `PlayerController.bShowMouseCursor` false (`GameplayStatics.GetPlayerController` 0))
              (`Widget.RemoveFromParent` (`self.PauseWidget`))
              (`KismetSystemLibrary.PrintString` "DeletePause")
              (else
                (bind _returnvalue (`|CreateWidget` "/Game/A_UI/WGT_PauseMenu.WGT_PauseMenu_C" (`GameplayStatics.GetPlayerController` 0)))
                (set `self.PauseWidget` _returnvalue)
                (`UserWidget.AddToViewport` _returnvalue 0)
                (`KismetSystemLibrary.PrintString` "CreatePause"))))
          (:`then_1`
            (`KismetSystemLibrary.Delay` 0.2)
            (goto _label :!via `Reset`)))))))

(fn `UserConstructionScript`)