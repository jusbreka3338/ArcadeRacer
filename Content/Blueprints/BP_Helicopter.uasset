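; BP_Helicopter is an invisible-logic or visible flyer that scatters BP_ItemBox pickups along landscape splines, starting at BeginPlay.
; SpawnHeli teleports it to a random XY at fixed altitude and line traces along its Arrow component.
; A LandscapeSplineActor hit spawns a box just above the impact and immediately repeats; any other result repeats after a short delay.
; The self-calling loop has no box limit or stop condition.
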(event `SpawnHeli`
  (bind _arrow (`self.Arrow`))
  (bind _returnvalue (`SceneComponent.K2_GetComponentLocation` _arrow))
  (`self.K2_SetActorLocationAndRotation` (`KismetMathLibrary.MakeVector` (`KismetMathLibrary.RandomFloatInRange` -100000.0 60000.0) (`KismetMathLibrary.RandomFloatInRange` -75000.0 50000.0) 25000.0))
  (bind _outhit (`KismetSystemLibrary.LineTraceSingle` _returnvalue (+ _returnvalue (* (`KismetMathLibrary.GetForwardVector` (`SceneComponent.K2_GetComponentRotation` _arrow)) 50000.0)) "TraceTypeQuery1"))
  (bind (_bblockinghit _binitialoverlap _time _distance _location _impactpoint _normal _impactnormal _physmat _hitactor) (`GameplayStatics.BreakHitResult` _outhit))
  (if (`.bSuccess` (cast `LandscapeSplineActor` _hitactor :!pure true))
    (`|SpawnActorFromClass` "/Game/Blueprints/BP_ItemBox.BP_ItemBox_C" (`KismetMathLibrary.MakeTransform` (+ _impactpoint (0.0 0.0 150.0))) "Undefined" "MultiplyWithRoot" null null)
    (`self.SpawnHeli`)
    (else
      (`KismetSystemLibrary.Delay` 0.5)
      (`self.SpawnHeli`))))

(event `self.ReceiveBeginPlay`
  (`self.SpawnHeli`))

(event `self.ReceiveTick`
  (params (DeltaSeconds :type "Float (single-precision)")))

(fn `UserConstructionScript`)