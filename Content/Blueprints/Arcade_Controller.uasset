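; Arcade_Controller is a player controller for the arcade game that sets up game-only input for local players.
; On BeginPlay, a local controller hides the mouse cursor and switches input mode to game only.
; A separate GetCharacterClas event copies four chosen-class values from the Arcade_GI game instance into the controller's own variables.
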(event `GetCharacterClas`
  (bind _asarcade_gi (cast `/Game/Blueprints/Arcade_GI` (`GameplayStatics.GetGameInstance`)))
  (set `self.Chosen Class` (`/Game/Blueprints/Arcade_GI.ChosenClass` _asarcade_gi))
  (set `self.Chosen Class 2` (`/Game/Blueprints/Arcade_GI.ChosenClass2` _asarcade_gi))
  (set `self.Chosen Class 3` (`/Game/Blueprints/Arcade_GI.ChosenClass3` _asarcade_gi))
  (set `self.Chosen Class 4` (`/Game/Blueprints/Arcade_GI.ChosenClass4` _asarcade_gi)))

(event `self.ReceiveBeginPlay`
  (if (`self.IsLocalPlayerController`)
    (set `self.bShowMouseCursor` false)
    (`WidgetBlueprintLibrary.SetInputMode_GameOnly` self)))

(fn `UserConstructionScript`)