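; Musics actor that crossfades between a Dream music track and a Normal music track.
; SwitchToDream and SwitchToNormal each play their own timeline from the start, ND and DN respectively.
; Each timeline update sets the volume multiplier on both audio components from its Dream and Normal curves.
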(event `SwitchToDream`
  (bind (_direction _normal _dream) (`Timeline|N-D` :!via `PlayFromStart`)
    (:`Update`
      (`AudioComponent.SetVolumeMultiplier` (`self.Dream`) _dream)
      (`AudioComponent.SetVolumeMultiplier` (`self.Normal`) _normal))))

(event `SwitchToNormal`
  (bind (_direction _normal _dream) (`Timeline|D-N` :!via `PlayFromStart`)
    (:`Update`
      (`AudioComponent.SetVolumeMultiplier` (`self.Dream`) _dream)
      (`AudioComponent.SetVolumeMultiplier` (`self.Normal`) _normal))))

(fn `UserConstructionScript`)