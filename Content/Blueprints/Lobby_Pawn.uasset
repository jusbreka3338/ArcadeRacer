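; Lobby pawn that displays a vehicle mesh, chosen by VehicleIndex, on its Scooter component.
; On BeginPlay, GetVehicleStats uses the index as a row name in Character_DT, stores the row as VehicleData, and applies its mesh, placement and rotation.
; The lookup runs only once, as the delayed repeat path is unreachable.
; A missing row only prints a placeholder debug string.
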(event `self.ReceiveBeginPlay`
  (`self.Get Vehicle Stats`)
  (`KismetSystemLibrary.Delay` 0.2))

(fn `Get Vehicle Stats`
  (locals (Vehicle_data :type "/Game/Blueprints/CharacterStruct Structure"))
  (bind _returnvalue (`|GetDataTableRow` "/Game/Blueprints/Character_DT.Character_DT" (`KismetStringLibrary.Conv_StringToName` (`KismetStringLibrary.Conv_IntToString` (`self.Vehicle_Index`))))
    (:`then`
      (bind _output_get (set `local.Vehicle_data` _returnvalue))
      (`StaticMeshComponent.SetStaticMesh` (`self.Scooter`) (break `/Game/Blueprints/CharacterStruct` _output_get))
      (`SceneComponent.K2_SetRelativeTransform` (`self.Scooter`) (`KismetMathLibrary.MakeTransform` (`.Placement_7_2CBB77407A43D610B6FA2EB47FD761A0` (break `/Game/Blueprints/CharacterStruct` _output_get)) (`.Rotation_8_7ACA9203F34FFF9F821A8698072B4ED1` (break `/Game/Blueprints/CharacterStruct` _output_get))) false false))
    (:`RowNotFound`
      (`KismetSystemLibrary.PrintString` "Hello"))))

(fn `UserConstructionScript`)