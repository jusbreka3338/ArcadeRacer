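; CustomPlayerController acts as a spawn point that moves a local player's vehicle to its own transform at game start, for up to four players.
; On BeginPlay it runs TeleportPlayers, but only if player 0's pawn is a BP_BaseVehicle.
; TeleportPlayers loops over every BP_BaseVehicle, matches its controller to player indices 0–3, and snaps the one matching PlayerSpawnIndex to the DefaultSceneRoot transform without sweeping.
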(event `self.ReceiveBeginPlay`
  (bind _asbp_scooter (cast `/Game/Blueprints/BP_BaseVehicle` (`GameplayStatics.GetPlayerPawn` 0)))
  (set `self.As BP Scooter` _asbp_scooter)
  (`self.Teleport Players`)
  (`KismetSystemLibrary.Delay` 0.2))

(event `self.ReceiveTick`
  (params (DeltaSeconds :type "Float (single-precision)")))

(event `Teleport Players`
  (bind _outactors (`GameplayStatics.GetAllActorsOfClass` "/Game/Blueprints/BP_BaseVehicle.BP_BaseVehicle_C"))
  (for _array_element _outactors
    (bind _returnvalue (`Pawn.GetController` _array_element))
    (if (== _returnvalue (`GameplayStatics.GetPlayerController` 0))
      (if (== (`self.PlayerSpawnIndex`) 0)
        (`self.K2_SetActorTransform` _array_element (`SceneComponent.K2_GetComponentToWorld` (`self.DefaultSceneRoot`)) false false))
      (elif (== _returnvalue (`GameplayStatics.GetPlayerController` 1))
        (if (== (`self.PlayerSpawnIndex`) 1)
          (`self.K2_SetActorTransform` _array_element (`SceneComponent.K2_GetComponentToWorld` (`self.DefaultSceneRoot`)) false false))
        (elif (== _returnvalue (`GameplayStatics.GetPlayerController` 2))
          (if (== (`self.PlayerSpawnIndex`) 2)
            (`self.K2_SetActorTransform` _array_element (`SceneComponent.K2_GetComponentToWorld` (`self.DefaultSceneRoot`)) false false))
          (elif (== _returnvalue (`GameplayStatics.GetPlayerController` 3))
            (if (== (`self.PlayerSpawnIndex`) 3)
              (`self.K2_SetActorTransform` _array_element (`SceneComponent.K2_GetComponentToWorld` (`self.DefaultSceneRoot`)) false false))))))))

(fn `UserConstructionScript`)