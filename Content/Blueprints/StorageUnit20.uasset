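; Item pickup and use system that holds one item and fires it on the ItemUse input.
; GetItem assigns an item, currently always Trash as the random range is pinned, or raises the held item's stage up to three.
; ItemUse spawns oil, pizza, trash or a delayed-flashbang firework by stage, then clears the slot.
; Only Oil handles all three stages; Cloud and Pillow have no use logic.
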(event `GetItem`
  (if (`KismetStringLibrary.EqualEqual_StrStr` (`self.ItemHeld`))
    (set `self.ItemStage` 1)
    (switch `int` (`KismetMathLibrary.RandomIntegerInRange` 3 3)
      (:`1`
        (set `self.ItemHeld` "Oil"))
      (:`2`
        (set `self.ItemHeld` "Pizza"))
      (:`3`
        (set `self.ItemHeld` "Trash"))
      (:`4`
        (set `self.ItemHeld` "Firework"))
      (:`5`
        (set `self.ItemHeld` "Cloud"))
      (:`6`
        (set `self.ItemHeld` "Pillow")))
    (elif (< (`self.ItemStage`) 3)
      (set `self.ItemStage` (+ (`self.ItemStage`) 1)))))

(event `InputAction|ItemUse`
  (params (Key :type "Key Structure"))
  (bind (_returnvalue_location _returnvalue_rotation) (`KismetMathLibrary.BreakTransform` (`SceneComponent.K2_GetComponentToWorld` (`self.OilSpawnLocation`))))
  (bind _returnvalue (`SceneComponent.K2_GetComponentToWorld` (`self.PizzaArrow`)))
  (bind (_returnvalue_location_2 _returnvalue_rotation_2) (`KismetMathLibrary.BreakTransform` (`SceneComponent.K2_GetComponentToWorld` (`self.PizzaArrow`))))
  (bind (_returnvalue_location_3 _returnvalue_rotation_3) (`KismetMathLibrary.BreakTransform` (`SceneComponent.K2_GetComponentToWorld` (`self.PizzaArrow`))))
  (bind (_returnvalue_location_4 _returnvalue_rotation_4) (`KismetMathLibrary.BreakTransform` (`SceneComponent.K2_GetComponentToWorld` (`self.OilSpawnLocation`))))
  (bind (_returnvalue_location_5 _returnvalue_rotation_5) (`KismetMathLibrary.BreakTransform` (`SceneComponent.K2_GetComponentToWorld` (`self.OilSpawnLocation`))))
  (bind (_returnvalue_location_6 _returnvalue_rotation_6) (`KismetMathLibrary.BreakTransform` (`SceneComponent.K2_GetComponentToWorld` (`self.OilSpawnLocation`))))
  (bind (_returnvalue_location_7 _returnvalue_rotation_7) (`KismetMathLibrary.BreakTransform` (`SceneComponent.K2_GetComponentToWorld` (`self.PizzaArrow`))))
  (bind (_returnvalue_location_8 _returnvalue_rotation_8) (`KismetMathLibrary.BreakTransform` (`SceneComponent.K2_GetComponentToWorld` (`self.PizzaArrow`))))
  (bind (_returnvalue_location_9 _returnvalue_rotation_9) (`KismetMathLibrary.BreakTransform` (`SceneComponent.K2_GetComponentToWorld` (`self.PizzaArrow`))))
  (bind (_returnvalue_location_10 _returnvalue_rotation_10) (`KismetMathLibrary.BreakTransform` (`SceneComponent.K2_GetComponentToWorld` (`self.PizzaArrow`))))
  (bind (_returnvalue_location_11 _returnvalue_rotation_11) (`KismetMathLibrary.BreakTransform` (`SceneComponent.K2_GetComponentToWorld` (`self.OilSpawnLocation`))))
  (bind (_returnvalue_location_12 _returnvalue_rotation_12) (`KismetMathLibrary.BreakTransform` (`SceneComponent.K2_GetComponentToWorld` (`self.OilSpawnLocation`))))
  (bind (_returnvalue_location_13 _returnvalue_rotation_13) (`KismetMathLibrary.BreakTransform` (`SceneComponent.K2_GetComponentToWorld` (`self.OilSpawnLocation`))))
  (bind (_returnvalue_location_14 _returnvalue_rotation_14) (`KismetMathLibrary.BreakTransform` (`SceneComponent.K2_GetComponentToWorld` (`self.OilSpawnLocation`))))
  (bind (_returnvalue_location_15 _returnvalue_rotation_15) (`KismetMathLibrary.BreakTransform` (`SceneComponent.K2_GetComponentToWorld` (`self.OilSpawnLocation`))))
  (bind (_returnvalue_location_16 _returnvalue_rotation_16) (`KismetMathLibrary.BreakTransform` (`SceneComponent.K2_GetComponentToWorld` (`self.OilSpawnLocation`))))
  (:`Pressed`
    (switch `string` (`self.ItemHeld`)
      (:`Oil`
        (switch `int` (`self.ItemStage`)
          (:`1`
            (`|SpawnActorFromClass` "/Game/Blueprints/BP_OilItem.BP_OilItem_C" (`KismetMathLibrary.MakeTransform` _returnvalue_location_4 _returnvalue_rotation_4) "Undefined" "MultiplyWithRoot" null null)
            (set `self.ItemHeld` "None")
            (set `self.ItemStage` 0))
          (:`2`
            (`|SpawnActorFromClass` "/Game/Blueprints/BP_OilItem.BP_OilItem_C" (`KismetMathLibrary.MakeTransform` _returnvalue_location_11 _returnvalue_rotation_11) "Undefined" "MultiplyWithRoot" null null)
            (`|SpawnActorFromClass` "/Game/Blueprints/BP_OilItem.BP_OilItem_C" (`KismetMathLibrary.MakeTransform` (+ _returnvalue_location_12 (600.0 -200.0 0.0)) _returnvalue_rotation_12) "Undefined" "MultiplyWithRoot" null null)
            (`|SpawnActorFromClass` "/Game/Blueprints/BP_OilItem.BP_OilItem_C" (`KismetMathLibrary.MakeTransform` (+ _returnvalue_location_13 (300.0 -600.0 0.0)) _returnvalue_rotation_13) "Undefined" "MultiplyWithRoot" null null)
            (set `self.ItemHeld` "None")
            (set `self.ItemStage` 0))
          (:`3`
            (`|SpawnActorFromClass` "/Game/Blueprints/BP_OilItem.BP_OilItem_C" (`KismetMathLibrary.MakeTransform` _returnvalue_location_5 _returnvalue_rotation_5) "Undefined" "MultiplyWithRoot" null null)
            (`|SpawnActorFromClass` "/Game/Blueprints/BP_OilItem.BP_OilItem_C" (`KismetMathLibrary.MakeTransform` (+ _returnvalue_location_14 (600.0 -200.0 0.0)) _returnvalue_rotation_14) "Undefined" "MultiplyWithRoot" null null)
            (`|SpawnActorFromClass` "/Game/Blueprints/BP_OilItem.BP_OilItem_C" (`KismetMathLibrary.MakeTransform` (+ _returnvalue_location (300.0 -600.0 0.0)) _returnvalue_rotation) "Undefined" "MultiplyWithRoot" null null)
            (`|SpawnActorFromClass` "/Game/Blueprints/BP_OilItem.BP_OilItem_C" (`KismetMathLibrary.MakeTransform` (+ _returnvalue_location_15 (100.0 700.0 0.0)) _returnvalue_rotation_15) "Undefined" "MultiplyWithRoot" null null)
            (`|SpawnActorFromClass` "/Game/Blueprints/BP_OilItem.BP_OilItem_C" (`KismetMathLibrary.MakeTransform` (+ _returnvalue_location_16 (900.0 100.0 0.0)) _returnvalue_rotation_16) "Undefined" "MultiplyWithRoot" null null)
            (`|SpawnActorFromClass` "/Game/Blueprints/BP_OilItem.BP_OilItem_C" (`KismetMathLibrary.MakeTransform` (+ _returnvalue_location_6 (-800.0 -400.0 0.0)) _returnvalue_rotation_6) "Undefined" "MultiplyWithRoot" null null)
            (set `self.ItemHeld` "None")
            (set `self.ItemStage` 0))))
      (:`Pizza`
        (switch `int` (`self.ItemStage`)
          (:`1`
            (`|SpawnActorFromClass` "/Game/Blueprints/BP_Pizza.BP_Pizza_C" (`KismetMathLibrary.MakeTransform` _returnvalue_location_7 _returnvalue_rotation_7) "Undefined" "MultiplyWithRoot" null null)
            (set `self.ItemHeld` "None")
            (set `self.ItemStage` 0))
          (:`2`
            (`|SpawnActorFromClass` "/Game/Blueprints/BP_Pizza.BP_Pizza_C" (`KismetMathLibrary.MakeTransform` _returnvalue_location_9 _returnvalue_rotation_9) "Undefined" "MultiplyWithRoot" null null)
            (`KismetSystemLibrary.Delay` 0.3)
            (`|SpawnActorFromClass` "/Game/Blueprints/BP_Pizza.BP_Pizza_C" (`KismetMathLibrary.MakeTransform` _returnvalue_location_8 _returnvalue_rotation_8) "Undefined" "MultiplyWithRoot" null null)
            (`KismetSystemLibrary.Delay` 0.3)
            (`|SpawnActorFromClass` "/Game/Blueprints/BP_Pizza.BP_Pizza_C" (`KismetMathLibrary.MakeTransform` _returnvalue_location_2 _returnvalue_rotation_2) "Undefined" "MultiplyWithRoot" null null)
            (set `self.ItemHeld` "None")
            (set `self.ItemStage` 0))))
      (:`Trash`
        (switch `int` (`self.ItemStage`)
          (:`1`
            (`|SpawnActorFromClass` "/Game/Blueprints/BP_TrashBag.BP_TrashBag_C" (`KismetMathLibrary.MakeTransform` _returnvalue_location_3 _returnvalue_rotation_3) "Undefined" "MultiplyWithRoot" null null)
            (set `self.ItemHeld` "None")
            (set `self.ItemStage` 0))
          (:`2`
            (`|SpawnActorFromClass` "/Game/Blueprints/BP_TrashBagBurst.BP_TrashBagBurst_C" (`KismetMathLibrary.MakeTransform` _returnvalue_location_10 _returnvalue_rotation_10) "Undefined" "MultiplyWithRoot" null null)
            (set `self.ItemHeld` "None")
            (set `self.ItemStage` 0))))
      (:`Firework`
        (switch `int` (`self.ItemStage`)
          (:`1`
            (bind _returnvalue_2 (`|SpawnActorFromClass` "/Game/Blueprints/BP_Firework.BP_Firework_C" (`KismetMathLibrary.MakeTransform` (.location _returnvalue) (`KismetMathLibrary.MakeRotator` (.roll (.rotation _returnvalue)) (+ (.pitch (.rotation _returnvalue)) 45.0) (.yaw (.rotation _returnvalue)))) "Undefined" "MultiplyWithRoot" null null))
            (set `self.ItemHeld` "None")
            (set `self.ItemStage` 0)
            (`KismetSystemLibrary.Delay` (`self.TimeBeforePop`))
            (`/Game/Blueprints/BP_Firework.Flashbang` _returnvalue_2 (`GameplayStatics.GetPlayerControllerID` null))))))))

(fn `UserConstructionScript`)