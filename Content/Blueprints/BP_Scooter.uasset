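; Player-driven arcade scooter with countdown-gated controls, drifting, camera look and a pause menu.
; Tick moves it kinematically, using speed-scaled steering and lean or DoDrift's time-ramped turn and mesh angle.
; A ground trace drives custom gravity, while four directional traces slow it and push it off walls.
; Obstacle overlaps play a spin-out unless dreaming; seven chained slipstream segments trail behind, though their overlap check does nothing.
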(event OnComponentBeginOverlap(Box)
  (params (OverlappedComponent :type Primitive%20Component%20Object%20Reference) (OtherActor :type Actor%20Object%20Reference) (OtherComp :type Primitive%20Component%20Object%20Reference) (OtherBodyIndex :type Integer) (bFromSweep :type Boolean) (SweepResult :type Hit%20Result%20Structure%20%28by%20ref%29))
  ;[1 0.4375 0.4375] Hitting Obstacle
  (Utilities|Casting|CastToBP_BaseObstacle OtherActor)
  (if (not (Variables|Default|GetisDreaming))
    (bind _spin (Timeline|ScooterSpin PlayFromStart)
      (:Update
        (Transformation|SetWorldRotation (Variables|Default|GetScooter) (Math|Rotator|MakeRotator 0.0 0.0 _spin) false false))
      (:Finished
        (Variables|Default|SetMaxSpeed (Variables|Default|GetMxSpd-Default))
        (Components|MoveComponentTo (Variables|Default|GetScooter) "0.000000,0.000000,-44.000000" "0.000000,90.000000,0.000000" false false 0.2 false)))))

(event Custom|Reset
  ;[1 0.5853 0.6654] Cameraing Stuff
  (Components|MoveComponentTo (Variables|Default|GetSpringArm) "0.000000,0.000000,200.000000" "-10.000000,0.000000,0.000000" false false 0.2 false))

(event EventBeginPlay
  ;[1 0.7014 0.08333] The Big Ones
  (Utilities|FlowControl|Sequence
    (:then_0
      ;[0.9909 0.6084 1] Physics Tick
      (Components|Tick|SetTickGroup "TG_DuringPhysics"))
    (:then_1
      ;[1 1 1] Arrays and Tags
      (Variables|Default|SetArrowDirections (Utilities|Array|MakeArray (Variables|Default|GetForward) (Variables|Default|GetRight) (Variables|Default|GetLeft) (Variables|Default|GetBackwards))))
    (:then_2
      (bind _outactors (Actor|GetAllActorswithTag "HitSafe")))
    (:then_3
      ;[1 1 1] Creating Ref to Game instance
      (bind _asarcade_gi (Utilities|Casting|CastToArcade_GI (Game|GetGameInstance)))
      (Variables|Default|SetArcade%20Game%20Instance _asarcade_gi))))

(event EventTick
  (params (DeltaSeconds :type Float%20%28single-precision%29))
  (bind _returnvalue (Transformation|GetActorLocation))
  (bind _slipseg4 (Variables|Default|GetSlipSeg4))
  (bind _drift (Variables|Default|GetDrift))
  (bind _slipseg1 (Variables|Default|GetSlipSeg1))
  (bind _slipseg5 (Variables|Default|GetSlipSeg5))
  (bind _slipseg2 (Variables|Default|GetSlipSeg2))
  (bind _slipseg3 (Variables|Default|GetSlipSeg3))
  (bind _slipseg6 (Variables|Default|GetSlipSeg6))
  (bind _slipseg7 (Variables|Default|GetSlipSeg7))
  (bind _box (Variables|Default|GetBox))
  (bind _arrow (Variables|Default|GetArrow))
  (bind _returnvalue_2 (Transformation|GetWorldRotation _drift))
  (bind _returnvalue_3 (Transformation|GetWorldLocation _arrow))
  ;[1 0.7014 0.08333] The Big Ones
  (Utilities|FlowControl|Sequence
    (:then_1
      ;[0.6929 0.5256 1] Movement
      (if (not (Variables|Default|GetDrifting))
        (CallFunction|InterpolateSteeringAngle (Variables|Default|GetSteeringInput) DeltaSeconds)
        (Transformation|AddActorWorldOffset (* DeltaSeconds (* (Transformation|GetActorForwardVector) (Variables|Default|GetCurrentSpeed))) true)
        (Transformation|SetActorRelativeRotation (Math|Rotator|MakeRotator (Math|Interpolation|FInterpTo (Variables|Default|GetCurrentLeanAngle) (* (Variables|Default|GetCurrentSteeringAngle) (Utilities|Operators|Divide (Variables|Default|GetCurrentSpeed) (Variables|Default|GetMaxSpeed) 1.0)) DeltaSeconds (Variables|Default|GetLeanSpeed)) 0.0 (+ (.yaw (Transformation|GetActorRotation)) (* (Variables|Default|GetCurrentSpeed) (Variables|Default|GetCurrentSteeringAngle) (Variables|Default|GetSpeedToRotationFactor) DeltaSeconds (Math|Float|SelectFloat 1.0 2.0 (< (Variables|Default|GetCurrentSpeed) 0.0))))))
        (Variables|Default|SetCurrentLeanAngle (* (Variables|Default|GetCurrentSteeringAngle) (Variables|Default|GetLeaningCoef)))
        (else
          (CallFunction|DoDrift DeltaSeconds))))
    (:then_2
      (Variables|Default|SetCurrentVelocity (+ (Variables|Default|GetCurrentVelocity) (* DeltaSeconds (Variables|Default|GetGravityValue)))))
    (:then_3
      ;[0.6296 0.8293 1] Gravity
      (bind _outhit (Collision|LineTraceByChannel _returnvalue_3 (+ _returnvalue_3 (* (Math|Vector|GetForwardVector (Transformation|GetWorldRotation _arrow)) 1.5e+03)) "TraceTypeQuery1" false 0 "None"))
      (Utilities|FlowControl|Sequence
        (:then_0
          (if (< (.z _returnvalue) (+ (.z (.Location (Collision|BreakHitResult _outhit))) 4e+01))
            (Transformation|SetActorLocation (Math|Vector|MakeVector (.x _returnvalue) (.y _returnvalue) (+ (.z (.Location (Collision|BreakHitResult _outhit))) 4e+01)) false false)
            (Variables|Default|SetCurrentVelocity 0.0)
            (else
              (Transformation|SetActorLocation (Math|Vector|MakeVector (.x _returnvalue) (.y _returnvalue) (+ (.z _returnvalue) (* (Variables|Default|GetCurrentVelocity) DeltaSeconds))) false false)
              (if (and (> (- (.z _returnvalue) (+ (.z (.Location (Collision|BreakHitResult _outhit))) 4e+01)) 1e+01) (not (Variables|Default|GetDrifting)))
                (if (Variables|Default|GetWasntFalling)
                  (Variables|Default|SetCurrentVelocity (|((y2-y1)/dt) (Variables|Default|GetPrevHitLocation) (Variables|Default|GetTwoFrameHitBuffer) DeltaSeconds))
                  (Variables|Default|SetWasntFalling false)
                  (Development|PrintString (Utilities|String|ToString(Float) (|((y2-y1)/dt) (Variables|Default|GetPrevHitLocation) (Variables|Default|GetTwoFrameHitBuffer) DeltaSeconds))))
                (else
                  (Variables|Default|SetWasntFalling true))))))
        (:then_1
          (Variables|Default|SetTwoFrameHitBuffer (Variables|Default|GetPrevHitLocation))
          (Variables|Default|SetPrevHitLocation (+ (.z (.Location (Collision|BreakHitResult _outhit))) 4e+01)))))
    (:then_5
      ;[1 0.5881 0.6531] Drift Rotation????
      (Transformation|SetWorldRotation (Variables|Default|GetDrift) (Math|Rotator|MakeRotator (.roll _returnvalue_2) 0.0 (.yaw _returnvalue_2)) false false))
    (:then_7
      ;[1 0.4328 0.2108] SlipDream Jambalaya
      (Utilities|FlowControl|Sequence
        (:then_0
          (Transformation|DetachFromComponent _slipseg1 "KeepRelative" "KeepRelative" "KeepRelative" true)
          (Components|MoveComponentTo _slipseg1 (Transformation|GetWorldLocation (Variables|Default|GetSlipStart)) "0, 0, 0" false false 0.05 false))
        (:then_1
          (Transformation|DetachFromComponent _slipseg2 "KeepRelative" "KeepRelative" "KeepRelative" true)
          (Components|MoveComponentTo _slipseg2 (Transformation|GetWorldLocation _slipseg1) "0, 0, 0" false false 0.05 false))
        (:then_2
          (Transformation|DetachFromComponent _slipseg3 "KeepRelative" "KeepRelative" "KeepRelative" true)
          (Components|MoveComponentTo _slipseg3 (Transformation|GetWorldLocation _slipseg2) "0, 0, 0" false false 0.05 false))
        (:then_3
          (Transformation|DetachFromComponent _slipseg4 "KeepRelative" "KeepRelative" "KeepRelative" true)
          (Components|MoveComponentTo _slipseg4 (Transformation|GetWorldLocation _slipseg3) "0, 0, 0" false false 0.05 false))
        (:then_4
          (Transformation|DetachFromComponent _slipseg5 "KeepRelative" "KeepRelative" "KeepRelative" true)
          (Components|MoveComponentTo _slipseg5 (Transformation|GetWorldLocation _slipseg4) "0, 0, 0" false false 0.05 false))
        (:then_5
          (Transformation|DetachFromComponent _slipseg6 "KeepRelative" "KeepRelative" "KeepRelative" true)
          (Components|MoveComponentTo _slipseg6 (Transformation|GetWorldLocation _slipseg5) "0, 0, 0" false false 0.05 false))
        (:then_6
          (Transformation|DetachFromComponent _slipseg7 "KeepRelative" "KeepRelative" "KeepRelative" true)
          (Components|MoveComponentTo _slipseg7 (Transformation|GetWorldLocation _slipseg6) "0, 0, 0" false false 0.05 false))))
    (:then_8
      ;[0.6929 0.6079 1] Slipdream Collision
      (if (Math|Boolean|ORBoolean (Class|PrimitiveComponent|IsOverlappingComponent _box (Variables|Default|GetSlipSeg1)) (Class|PrimitiveComponent|IsOverlappingComponent _box (Variables|Default|GetSlipSeg2)) (Class|PrimitiveComponent|IsOverlappingComponent _box (Variables|Default|GetSlipSeg3)) (Class|PrimitiveComponent|IsOverlappingComponent _box (Variables|Default|GetSlipSeg4)) (Class|PrimitiveComponent|IsOverlappingComponent _box (Variables|Default|GetSlipSeg5)) (Class|PrimitiveComponent|IsOverlappingComponent _box (Variables|Default|GetSlipSeg6)) (Class|PrimitiveComponent|IsOverlappingComponent _box (Variables|Default|GetSlipSeg7)))
        _))
    (:then_10
      ;[0.9212 0.722 1] Wall Detection
      (for (_array_element _array_index) (Variables|Default|GetArrowDirections)
        (switch int _array_index
          (:0
            (Variables|Default|SetWallDetectionDrawDistance 1e+02 :!label _label))
          (:1
            (Variables|Default|SetWallDetectionDrawDistance 5e+01 :!label _label_2))
          (:2
            (goto _label_2))
          (:3
            (goto _label)))
        (bind (_outhit_2 _returnvalue_4) (Collision|LineTraceByChannel (Transformation|GetWorldLocation _array_element) (+ (Transformation|GetWorldLocation _array_element) (* (Math|Vector|GetForwardVector (Transformation|GetWorldRotation _array_element)) (Variables|Default|GetWallDetectionDrawDistance))) "TraceTypeQuery1" false (stale EventBeginPlay _outactors) "None"))
        (if _returnvalue_4
          (Variables|Default|SetCurrentSpeed (* (Variables|Default|GetCurrentSpeed) (|(1-a) (Math|Float|Absolute(Float) (Math|Vector|DotProduct (.Normal (Collision|BreakHitResult _outhit_2)) (Math|Vector|GetForwardVector (Variables|Default|GetForward)))))))
          (Transformation|SetActorLocation (+ (Transformation|GetActorLocation) (* (.Normal (Collision|BreakHitResult _outhit_2)) "2.000000,2.000000,0.000000")) false false))))))

(event Input|ActionEvents|InputActionPauseMenu
  (params (Key :type Key%20Structure))
  (bind _arcade_game_instance (Variables|Default|GetArcade%20Game%20Instance))
  ;[1 1 1] PauseStuff
  (:Pressed
    (Utilities|FlowControl|DoOnce false :!label _label
      (:Completed
        (Utilities|FlowControl|Sequence
          (:then_0
            (if (Variables|/Game/Blueprints/Arcade_GI.Arcade_GI_C|GetIsInPauseMenu? _arcade_game_instance)
              (Variables|/Game/Blueprints/Arcade_GI.Arcade_GI_C|SetIsInPauseMenu? _arcade_game_instance false)
              (Input|SetInputModeGameOnly 0 false)
              (Variables|/Script/Engine.PlayerController|SetbShowMouseCursor (Game|GetPlayerController 0) false)
              (Widget|RemovefromParent (Variables|Default|GetPauseWidget))
              (else
                (bind _returnvalue (UserInterface|CreateWidget "/Game/A_UI/WGT_PauseMenu.WGT_PauseMenu_C" (Game|GetPlayerController 0)))
                (Variables|Default|SetPauseWidget _returnvalue)
                (UserInterface|Viewport|AddtoViewport _returnvalue 0))))
          (:then_1
            (Utilities|FlowControl|Delay 0.2)
            (goto _label Reset)))))))

(event Input|ActionEvents|InputActionDrift
  (params (Key :type Key%20Structure))
  (:Pressed
    (Variables|Default|SetDrifting true)
    (Variables|Default|SetTurnInterpolation 0.5)
    (Variables|Default|SetCurrentSteeringAngle 0.0)
    (Variables|Default|SetCurrentLeanAngle 0.0)
    (Variables|Default|SetDriftTime 0.0))
  (:Released
    (Variables|Default|SetDrifting false)
    (Transformation|SetRelativeRotation (Variables|Default|GetScooter) "0.000000,90.000000,0.000000" false false)))

(event Input|ActionEvents|InputActionPhysics
  (params (Key :type Key%20Structure))
  (bind _scooter (Variables|Default|GetScooter))
  ;[1 0.6915 0.5183] How Hungry?
  (:Pressed
    (Utilities|FlowControl|FlipFlop
      (:A
        (Physics|SetSimulatePhysics _scooter true))
      (:B
        (Physics|SetSimulatePhysics _scooter false)))))

(event Input|ActionEvents|InputActionResetCamera
  (params (Key :type Key%20Structure))
  ;[1 0.5853 0.6654] Cameraing Stuff
  (:Pressed
    (if (Variables|Default|Getcountdownover?)
      _
      (else
        _))
    (if (not (Variables|/Game/Blueprints/Arcade_GI.Arcade_GI_C|GetIsInPauseMenu? (Variables|Default|GetArcade%20Game%20Instance)))
      (Components|MoveComponentTo (Variables|Default|GetSpringArm) "0.000000,0.000000,200.000000" "-10.000000,0.000000,0.000000" false false 0.2 false))))

(event Input|ActionEvents|InputActionReadycountDown
  (params (Key :type Key%20Structure))
  ;[1 1 1] Ready Up
  (:Pressed
    (bind _asarcade_gm (Utilities|Casting|CastToArcade_GM (Game|GetGameMode)))
    (if (not (Variables|/Game/Blueprints/Arcade_GM.Arcade_GM_C|GetCountdownover _asarcade_gm))
      (if (>= (Variables|/Game/Blueprints/Arcade_GM.Arcade_GM_C|GetStartCountdownDuration _asarcade_gm) 3.500001)
        (Variables|/Game/Blueprints/Arcade_GM.Arcade_GM_C|SetStartCountdownDuration _asarcade_gm 3.5)
        (Default|StartCountdown _asarcade_gm)))))

(event Input|ActionEvents|InputActionReadycountDown
  (params (Key :type Key%20Structure))
  ;[1 1 1] Ready Up
  (:Pressed
    (bind _asarcade_gm (Utilities|Casting|CastToArcade_GM (Game|GetGameMode)))
    (if (not (Variables|/Game/Blueprints/Arcade_GM.Arcade_GM_C|GetCountdownover _asarcade_gm))
      (if (>= (Variables|/Game/Blueprints/Arcade_GM.Arcade_GM_C|GetStartCountdownDuration _asarcade_gm) 3.500001)
        (Variables|/Game/Blueprints/Arcade_GM.Arcade_GM_C|SetStartCountdownDuration _asarcade_gm 3.5)
        (Default|StartCountdown _asarcade_gm)))))

(event Input|AxisEvents|InputAxisThrottle
  (params (AxisValue :type Float%20%28single-precision%29))
  (bind _returnvalue (Math|Float|Clamp(Float) AxisValue -0.25))
  ;[0.7561 1 0.7271] Movement Inputs
  (if (and (Variables|Default|Getcountdownover?) (not (Variables|/Game/Blueprints/Arcade_GI.Arcade_GI_C|GetIsInPauseMenu? (Variables|Default|GetArcade%20Game%20Instance))))
    (Variables|Default|SetCurrentSpeed (Math|Interpolation|FInterpTo (Variables|Default|GetCurrentSpeed) (* _returnvalue (Variables|Default|GetMaxSpeed)) (Utilities|Time|GetWorldDeltaSeconds) (Math|Float|SelectFloat 1.0 0.8 (> _returnvalue 0.0))))))

(event Input|AxisEvents|InputAxisSteer
  (params (AxisValue :type Float%20%28single-precision%29))
  ;[0.7561 1 0.7271] Movement Inputs
  (if (and (Variables|Default|Getcountdownover?) (not (Variables|/Game/Blueprints/Arcade_GI.Arcade_GI_C|GetIsInPauseMenu? (Variables|Default|GetArcade%20Game%20Instance))))
    (Variables|Default|SetSteeringInput AxisValue)))

(event Input|AxisEvents|InputAxisLookRight
  (params (AxisValue :type Float%20%28single-precision%29))
  ;[1 0.5853 0.6654] Cameraing Stuff
  (if (not (Variables|Default|Getcountdownover?))
    (if (not (Variables|/Game/Blueprints/Arcade_GI.Arcade_GI_C|GetIsInPauseMenu? (Variables|Default|GetArcade%20Game%20Instance)))
      (Transformation|AddRelativeRotation (Variables|Default|GetSpringArm) (Math|Rotator|MakeRotator 0.0 0.0 AxisValue) false false))))

(event Input|AxisEvents|InputAxisLookUp
  (params (AxisValue :type Float%20%28single-precision%29))
  ;[1 0.5853 0.6654] Cameraing Stuff
  (if (not (Variables|Default|Getcountdownover?))
    (if (not (Variables|/Game/Blueprints/Arcade_GI.Arcade_GI_C|GetIsInPauseMenu? (Variables|Default|GetArcade%20Game%20Instance)))
      (Transformation|AddRelativeRotation (Variables|Default|GetSpringArm) (Math|Rotator|MakeRotator 0.0 AxisValue 0.0) false false))))

(fn ConstructionScript)

(fn InterpolateSteeringAngle
  (params (InputDir :type Float%20%28double-precision%29) (DeltaTime :type Float%20%28double-precision%29))
  (bind _maxsteeringangle (Variables|Default|GetMaxSteeringAngle))
  (bind _minsteeringangle (Variables|Default|GetMinSteeringAngle))
  (bind _currentspeed (Variables|Default|GetCurrentSpeed))
  (bind _maxspeed (Variables|Default|GetMaxSpeed))
  (bind _returnvalue (/ _currentspeed _maxspeed))
  (bind _returnvalue_2 (Math|Float|Clamp(Float) _returnvalue))
  (bind _returnvalue_3 (Math|Float|Lerp _maxsteeringangle _minsteeringangle _returnvalue_2))
  (bind _output_get (Variables|Default|SetTurnInterpolation (+ (Variables|Default|GetTurnInterpolation) (* (- (|((a+1)/2) InputDir) (Variables|Default|GetTurnInterpolation)) (Math|Float|SelectFloat (Variables|Default|GetReturnTurnSpeed) (Variables|Default|GetTurnSpeed) (== (Variables|Default|GetSteeringInput) 0.0)) DeltaTime))))
  (Variables|Default|SetCurrentSteeringAngle (Math|Float|Lerp (* _returnvalue_3 -1.0) _returnvalue_3 _output_get)))

(fn DoDrift
  (params (DeltaTime :type Float%20%28double-precision%29))
  (bind _returnvalue (Transformation|GetActorRotation))
  (bind _returnvalue_2 (Transformation|GetActorRotation))
  (bind _scooter (Variables|Default|GetScooter))
  (bind _returnvalue_3 (Transformation|GetWorldRotation _scooter))
  (bind _returnvalue_4 (- (.yaw _returnvalue_3) (.yaw _returnvalue)))
  (bind _returnvalue_5 (> _returnvalue_4 0.0))
  (bind _returnvalue_6 (+ _returnvalue_4 3.6e+02))
  (bind _returnvalue_7 (Math|Float|SelectFloat _returnvalue_4 _returnvalue_6 _returnvalue_5))
  (Variables|Default|SetDriftTime (+ (Variables|Default|GetDriftTime) DeltaTime))
  (Transformation|SetActorRelativeRotation (Math|Rotator|MakeRotator (- (.roll _returnvalue_2) (* (.roll _returnvalue_2) DeltaTime (Variables|Default|GetDriftAngleSpeed))) (.pitch _returnvalue_2) (+ (.yaw _returnvalue_2) (* (Variables|Default|GetSteeringInput) (Variables|Default|GetDriftSpeed) (Math|Float|Clamp(Float) (/ (Variables|Default|GetDriftTime) (Variables|Default|GetDriftTimeMax))) DeltaTime))))
  (Transformation|AddActorWorldOffset (* (Transformation|GetActorForwardVector) (* (Variables|Default|GetCurrentSpeed) DeltaTime)) true)
  (Transformation|SetRelativeRotation (Variables|Default|GetScooter) (Math|Rotator|MakeRotator 0.0 0.0 (+ (* (- (+ (* (Variables|Default|GetSteeringInput) (Variables|Default|GetDriftAngle) (Math|Float|Clamp(Float) (/ (Variables|Default|GetDriftTime) (Variables|Default|GetDriftTimeMax)))) 9e+01) _returnvalue_7) (Variables|Default|GetDriftAngleSpeed) DeltaTime) _returnvalue_7)) false false))