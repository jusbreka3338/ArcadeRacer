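; BP_DumpsterObstacle is a dumpster hazard that bursts open and launches trash when a BP_Scooter enters its trigger box.
; The overlap quickly swings the hinge component with MoveComponentTo and, after a short delay, a DoOnce turns on physics for two trash pieces.
; Each piece gets an upward velocity-change impulse, then a delayed sideways one.
; A scooter overlapping either piece calls its SpinOut.
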(event `self.Box.OnComponentBeginOverlap`
  (params (OverlappedComponent :type "PrimitiveComponent Object Reference") (OtherActor :type "Actor Object Reference") (OtherComp :type "PrimitiveComponent Object Reference") (OtherBodyIndex :type Integer) (bFromSweep :type Boolean) (SweepResult :type "HitResult Structure (by ref)"))
  (bind _trash2 (`self.Trash2`))
  (bind _trash1 (`self.Trash1`))
  (cast `/Game/Blueprints/BP_Scooter` OtherActor)
  (`|ExecutionSequence`
    (:`then_0`
      (`KismetSystemLibrary.MoveComponentTo` (`self.DumpsterHinge`) (0.0 122.0 174.0) (struct :`Roll` 90.0) false false 0.1))
    (:`then_1`
      (`KismetSystemLibrary.Delay` 0.05)
      (`/Engine/EditorBlueprintResources/StandardMacros.DoOnce` false
        (:`Completed`
          (`|ExecutionSequence`
            (:`then_0`
              (`PrimitiveComponent.SetSimulatePhysics` _trash1 true)
              (`PrimitiveComponent.AddImpulse` _trash1 (100.0 0.0 1500.0) "None" true)
              (`KismetSystemLibrary.Delay` 0.2)
              (`PrimitiveComponent.AddImpulse` _trash1 (0.0 750.0 0.0) "None" true))
            (:`then_1`
              (`PrimitiveComponent.SetSimulatePhysics` _trash2 true)
              (`PrimitiveComponent.AddImpulse` _trash2 (-100.0 0.0 1500.0) "None" true)
              (`KismetSystemLibrary.Delay` 0.2)
              (`PrimitiveComponent.AddImpulse` _trash2 (0.0 750.0 0.0) "None" true))))))))

(event `self.Trash1.OnComponentBeginOverlap`
  (params (OverlappedComponent :type "PrimitiveComponent Object Reference") (OtherActor :type "Actor Object Reference") (OtherComp :type "PrimitiveComponent Object Reference") (OtherBodyIndex :type Integer) (bFromSweep :type Boolean) (SweepResult :type "HitResult Structure (by ref)"))
  (bind _asbp_scooter (cast `/Game/Blueprints/BP_Scooter` OtherActor))
  (`/Game/Blueprints/BP_Scooter.SpinOut` _asbp_scooter null))

(event `self.Trash2.OnComponentBeginOverlap`
  (params (OverlappedComponent :type "PrimitiveComponent Object Reference") (OtherActor :type "Actor Object Reference") (OtherComp :type "PrimitiveComponent Object Reference") (OtherBodyIndex :type Integer) (bFromSweep :type Boolean) (SweepResult :type "HitResult Structure (by ref)"))
  (bind _asbp_scooter (cast `/Game/Blueprints/BP_Scooter` OtherActor))
  (`/Game/Blueprints/BP_Scooter.SpinOut` _asbp_scooter null))

(fn `UserConstructionScript`)