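; A placeable manager actor that registers the spawn points for up to four players in the arcade game mode.
; On BeginPlay it casts the game mode to Arcade_GM and copies the transforms of four PlayerStart array entries into its Player1Start through Player4Start variables.
; If the cast fails it does nothing, as the delay and failure-print nodes are left unconnected.
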(event `self.ReceiveBeginPlay`
  (bind _playerstart (`self.PlayerStart`))
  (bind _asarcade_gm (cast `/Game/Blueprints/Arcade_GM` (`GameplayStatics.GetGameMode`)))
  (set `/Game/Blueprints/Arcade_GM.Player1Start` (`self.GetTransform` (`|GetArrayItem` _playerstart)) _asarcade_gm)
  (set `/Game/Blueprints/Arcade_GM.Player2Start` (`self.GetTransform` (`|GetArrayItem` _playerstart 1)) _asarcade_gm)
  (set `/Game/Blueprints/Arcade_GM.Player3Start` (`self.GetTransform` (`|GetArrayItem` _playerstart 2)) _asarcade_gm)
  (set `/Game/Blueprints/Arcade_GM.Player4Start` (`self.GetTransform` (`|GetArrayItem` _playerstart 3)) _asarcade_gm))

(fn `UserConstructionScript`)