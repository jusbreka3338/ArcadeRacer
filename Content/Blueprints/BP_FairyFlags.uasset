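; BP_FairyFlags is a decorative string of flags that hangs from a simulated Cable component and follows its motion.
; On BeginPlay it adds one static mesh component per cable particle at that particle's location and stores it in the Flags array.
; Every Tick it moves each flag to the current world location of its matching particle, updating position only, so the flags do not rotate with the cable.
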(event `self.ReceiveBeginPlay`
  (bind _locations (`CableComponent.GetCableParticleLocations` (`self.Cable`)))
  (for (_ _array_index) _locations
    (bind _returnvalue (`AddComponent|NODE_AddStaticMeshComponent-0` :`bManualAttachment` true :`RelativeTransform` (`KismetMathLibrary.MakeTransform` (`|GetArrayItem` _locations _array_index))))
    (`KismetArrayLibrary.Array_Add` (`self.Flags`) _returnvalue)))

(event `self.ReceiveTick`
  (params (DeltaSeconds :type "Float (single-precision)"))
  (for (_array_element _array_index) (`self.Flags`)
    (`SceneComponent.K2_SetWorldLocation` _array_element (`|GetArrayItem` (`CableComponent.GetCableParticleLocations` (`self.Cable`)) _array_index) false false)))

(fn `UserConstructionScript`)