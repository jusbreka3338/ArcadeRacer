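; Lobby spawn marker, despite its controller name, that snaps the pawn of the player matching its PlayerSpawnIndex to its root transform.
; On BeginPlay it caches Lobby_GM, then TeleportPlayers compares each Lobby_Pawn's controller against the first four player controllers, with debug prints.
; The fourth-player branch transforms this actor itself rather than the pawn.
; Scooter-cast chains are leftovers that never run.
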(event `CustomEvent`)

(event `self.ReceiveBeginPlay`
  (bind _aslobby_gm (cast `/Game/Blueprints/Lobby_GM` (`GameplayStatics.GetGameMode`)))
  (set `self.As Lobby GM` _aslobby_gm)
  (`self.Teleport Players`)
  (`KismetSystemLibrary.Delay` 0.2))

(event `Teleport Players`
  (bind _outactors (`GameplayStatics.GetAllActorsOfClass` "/Game/Blueprints/Lobby_Pawn.Lobby_Pawn_C"))
  (for _array_element _outactors
    (bind _returnvalue (`Pawn.GetController` _array_element))
    (if (== _returnvalue (`GameplayStatics.GetPlayerController` 0))
      (`KismetSystemLibrary.PrintString` "Player1")
      (if (== (`self.PlayerSpawnIndex`) 0)
        (`self.K2_SetActorTransform` _array_element (`SceneComponent.K2_GetComponentToWorld` (`self.DefaultSceneRoot`)) false false))
      (elif (== _returnvalue (`GameplayStatics.GetPlayerController` 1))
        (`KismetSystemLibrary.PrintString` "Player2")
        (if (== (`self.PlayerSpawnIndex`) 1)
          (`self.K2_SetActorTransform` _array_element (`SceneComponent.K2_GetComponentToWorld` (`self.DefaultSceneRoot`)) false false))
        (elif (== _returnvalue (`GameplayStatics.GetPlayerController` 2))
          (`KismetSystemLibrary.PrintString` "Player3")
          (if (== (`self.PlayerSpawnIndex`) 2)
            (`self.K2_SetActorTransform` _array_element (`SceneComponent.K2_GetComponentToWorld` (`self.DefaultSceneRoot`)) false false))
          (elif (== _returnvalue (`GameplayStatics.GetPlayerController` 3))
            (`KismetSystemLibrary.PrintString` "Player4")
            (if (== (`self.PlayerSpawnIndex`) 3)
              (`self.K2_SetActorTransform` (`SceneComponent.K2_GetComponentToWorld` (`self.DefaultSceneRoot`))))
            (else
              (`KismetSystemLibrary.PrintString` "NOPE\n"))))))))

(fn `UserConstructionScript`)