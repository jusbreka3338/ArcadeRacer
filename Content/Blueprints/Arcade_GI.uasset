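; Arcade game instance that keeps the player's profile across sessions and opens the main menu.
; On init it loads the Arcade_SG save from the profile slot or creates one, and saves again whenever the player name changes.
; The menu function reuses or creates the widget, enables the cursor and fills in the saved name.
; SetTags is empty, and the scooter player-tagging logic for four local players is disconnected.
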(event `self.ReceiveInit`
  (`self.CheckForSavedProfile`))

(event `SetTags`)

(event `Change_PlayerName`
  (params (PlayerName :type Text))
  (set `self.Player Profile_Info` (make `/Game/Blueprints/S_PlayerProfiel` PlayerName))
  (`self.SaveProfile`))

(fn `CheckForSavedProfile`
  (bind _returnvalue (`GameplayStatics.DoesSaveGameExist` (`self.PlayerProfile_Slot`)))
  (if _returnvalue
    (bind _asarcade_sg (`self.LoadProfile`))
    (set `self.SG_PlayerProfile` _asarcade_sg)
    (else
      (`self.SaveProfile`)))
  (return))

(fn `LoadProfile`
  (returns (`AsArcade SG` :type "/Game/Blueprints/Arcade_SG Object Reference"))
  (bind _returnvalue (`GameplayStatics.LoadGameFromSlot` (`self.PlayerProfile_Slot`)))
  (bind _asarcade_sg (cast `/Game/Blueprints/Arcade_SG` _returnvalue))
  (set `self.Player Profile_Info` (`/Game/Blueprints/Arcade_SG.PlayerProfile` _asarcade_sg))
  (return _asarcade_sg))

(fn `SaveProfile`
  (bind _sg_playerprofile (`self.SG_PlayerProfile`))
  (`/Engine/EditorBlueprintResources/StandardMacros.IsValid` (`self.SG_PlayerProfile`)
    (:`Is Valid`
      _)
    (:`Is Not Valid`
      (bind _returnvalue (`GameplayStatics.CreateSaveGameObject` "/Game/Blueprints/Arcade_SG.Arcade_SG_C"))
      (set `self.SG_PlayerProfile` _returnvalue)))
  (set `/Game/Blueprints/Arcade_SG.PlayerProfile` (`self.Player Profile_Info`) _sg_playerprofile)
  (`GameplayStatics.SaveGameToSlot` _sg_playerprofile (`self.PlayerProfile_Slot`))
  (return))

(fn `UI_ShowMainMenu`
  (bind _returnvalue (`GameplayStatics.GetPlayerController` 0))
  (`/Engine/EditorBlueprintResources/StandardMacros.IsValid` (`self.WGT MainMenu`)
    (:`Is Valid`
      _)
    (:`Is Not Valid`
      (bind _returnvalue_2 (`|CreateWidget` "/Game/A_UI/WGT_MM.WGT_MM_C" _returnvalue))
      (set `self.WGT MainMenu` _returnvalue_2)))
  (`UserWidget.AddToViewport` (`self.WGT MainMenu`) 0)
  (`WidgetBlueprintLibrary.SetInputMode_GameAndUIEx` _returnvalue _returnvalue_2)
  (set `PlayerController.bShowMouseCursor` true _returnvalue)
  (`self.CheckForSavedProfile`)
  (`EditableText.SetText` (`/Game/A_UI/WGT_MM.Input_Playername` (`self.WGT MainMenu`)) (`.PlayerName_2_9773E1BF674272B22BCED0A95AEDF697` (break `/Game/Blueprints/S_PlayerProfiel` (`self.Player Profile_Info`))))
  (return))