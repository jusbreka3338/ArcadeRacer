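; Main menu pawn that lets gamepad input nudge the mouse cursor.
; A thumbstick axis event offsets the player controller's mouse location by scaled axis values.
; Tick, throttled by a short Delay, copies an axis value into the right-trigger field of the cached Arcade_GI game instance.
; The MainMenuNavigater action only prints debug text, and disconnected experiments for widget creation and simulated clicks never run.
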(event `self.ReceiveBeginPlay`
  (bind _asarcade_gi (cast `/Game/Blueprints/Arcade_GI` (`GameplayStatics.GetGameInstance`)))
  (set `self.As Arcade GI` _asarcade_gi))

(event `self.ReceiveTick`
  (params (DeltaSeconds :type "Float (single-precision)"))
  (`KismetSystemLibrary.Delay` 0.2)
  (set `/Game/Blueprints/Arcade_GI.ValueOfRightTrigger` (`self.GetInputAxisKeyValue`) (`self.As Arcade GI`)))

(event `InputAxisKey|Gamepad_LeftY`
  (params (AxisValue :type "Float (single-precision)")))

(event `InputAxis|NINputAxisTHUMBY`
  (params (AxisValue :type "Float (single-precision)"))
  (bind (_locationx _locationy) (`PlayerController.GetMousePosition` (`GameplayStatics.GetPlayerController` 0)))
  (`PlayerController.SetMouseLocation` (`GameplayStatics.GetPlayerController` 0) (`KismetMathLibrary.Round` (+ (* (`self.GetInputAxisKeyValue`) 10.0) _locationx)) (`KismetMathLibrary.Round` (+ _locationy (* (`self.GetInputAxisKeyValue`) 10.0)))))

(event `InputAction|MainMenuNavigater`
  (params (Key :type "Key Structure"))
  (:`Pressed`
    (`KismetSystemLibrary.PrintString` "HIT"))
  (:`Released`
    (`KismetSystemLibrary.PrintString` "RELEASE")))

(fn `UserConstructionScript`)