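; TempPawn is a pawn that moves a sticker between posters on walls using Left and Right axis input, gated by the DoStuff flag for ready-up.
; GetInputL and GetInputR apply a threshold and DoOnce latch, each decrementing the Poster index modulo 4.
; CalculateOffset supplies the teleport location and rotation on input and BeginPlay, with poster-transform math left unconnected.
; Tick switches Yoffset according to the Poster index.
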(event `InputAxis|Left`
  (params (AxisValue :type "Float (single-precision)"))
  ;[0.5605 0.7698 1] Manages Sticker Movement
  ;;[1 0.5134 0.5582] Seperate event based on direction
  (if (`self.DoStuff`)
    ;;[1 1 1] Gets Input and Creates Deadzone To Control Sticker Movement
    (bind _output_get (`self.Get Input R` AxisValue))
    (bind (_returnvalue _returnvalue2 _returnvalue3 _returnvalue4) (`self.Calculate Offset` _output_get))
    ;;[0.5687 0.6589 1] Actual Movement
    (`self.K2_SetActorLocation` (`KismetMathLibrary.MakeVector` _returnvalue _returnvalue2 _returnvalue3) false true)
    (`self.K2_SetActorRotation` _returnvalue4)))

(event `self.ReceiveBeginPlay`
  ;[0.5605 0.7698 1] Manages Sticker Movement
  (bind (_returnvalue _returnvalue2 _returnvalue3 _returnvalue4) (`self.Calculate Offset` (stale `InputAxis|Right` _output_get)))
  ;;[0.5687 0.6589 1] Actual Movement
  (`self.K2_SetActorLocation` (`KismetMathLibrary.MakeVector` _returnvalue _returnvalue2 _returnvalue3) false true :!label _label)
  (`self.K2_SetActorRotation` _returnvalue4))

(event `InputAxis|Right`
  (params (AxisValue :type "Float (single-precision)"))
  ;[0.5605 0.7698 1] Manages Sticker Movement
  ;;[1 0.5134 0.5582] Seperate event based on direction
  (if (`self.DoStuff`)
    ;;[1 1 1] Gets Input and Creates Deadzone To Control Sticker Movement
    (bind _output_get (`self.Get Input L` AxisValue))
    (goto _label)))

(event `self.ReceiveTick`
  (params (DeltaSeconds :type "Float (single-precision)"))
  ;[0.5605 0.7698 1] Manages Sticker Movement
  ;;[0.6281 1 0.6717] Manages Offset When Switching Walls
  (if (>= (`self.poster`) 1)
    (set `self.yoffset` 0.0)
    (else
      (set `self.yoffset` 50.0))))

(fn `UserConstructionScript`)