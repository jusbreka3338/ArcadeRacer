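; BP_CheckPoint is a vehicle checkpoint actor with a query-only cylinder trigger that looks up BP_CheckpointManager shortly after BeginPlay.
; Its overlap event is empty, leaving the progression logic disconnected.
; That dead logic compares CheckpointWanted with BP_BaseVehicle's CheckpointRequired to register hits or show a wrong-checkpoint arrow.
; Counter increments, hiding and progress-text updates are also unreachable, and CheckpointsToText has its formatting unwired.
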(event `self.ReceiveBeginPlay`
  (`PrimitiveComponent.SetCollisionEnabled` (`self.Cylinder`) "QueryOnly")
  (`KismetSystemLibrary.Delay` 0.2)
  (bind _returnvalue (`GameplayStatics.GetActorOfClass` "/Game/Blueprints/BP_CheckpointManager.BP_CheckpointManager_C"))
  (set `self.CheckpointManager` _returnvalue))

(event `self.Cylinder.OnComponentBeginOverlap`
  (params (OverlappedComponent :type "PrimitiveComponent Object Reference") (OtherActor :type "Actor Object Reference") (OtherComp :type "PrimitiveComponent Object Reference") (OtherBodyIndex :type Integer) (bFromSweep :type Boolean) (SweepResult :type "HitResult Structure (by ref)")))

(fn `UserConstructionScript`)