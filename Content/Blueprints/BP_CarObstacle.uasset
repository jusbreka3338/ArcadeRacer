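; Car obstacle that breaks into loose physics pieces when a BP_BaseVehicle overlaps its Box trigger.
; The overlap turns on physics for the car mesh and both doors and plays one of two random sounds, a clown toot or a boom.
; A DoOnce gates the reaction and re-arms after a short delay, though physics is never switched back off.
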(event `self.Box.OnComponentBeginOverlap`
  (params (OverlappedComponent :type "PrimitiveComponent Object Reference") (OtherActor :type "Actor Object Reference") (OtherComp :type "PrimitiveComponent Object Reference") (OtherBodyIndex :type Integer) (bFromSweep :type Boolean) (SweepResult :type "HitResult Structure (by ref)"))
  (bind _returnvalue_location (`KismetMathLibrary.BreakTransform` (`SceneComponent.GetRelativeTransform` (`self.CarMesh`))))
  (cast `/Game/Blueprints/BP_BaseVehicle` OtherActor)
  (`/Engine/EditorBlueprintResources/StandardMacros.DoOnce` false :!label _label
    (:`Completed`
      (`PrimitiveComponent.SetSimulatePhysics` (`self.CarMesh`) true)
      (`|ExecutionSequence`
        (:`then_0`
          (switch `int` (`KismetMathLibrary.RandomIntegerInRange` 1 2)
            (:`1`
              (`GameplayStatics.PlaySoundAtLocation` "/Game/Sound/Obstacles/car_clown_toot.car_clown_toot" (0.0 0.0 0.0) (struct) 1.0 1.0 0.0 null null null null))
            (:`2`
              (`GameplayStatics.PlaySoundAtLocation` "/Game/Sound/Obstacles/car_boom.car_boom" _returnvalue_location (struct) 1.0 1.0 0.0 null null null null))))
        (:`then_1`
          (`PrimitiveComponent.SetSimulatePhysics` (`self.LeftDoor`) true)
          (`PrimitiveComponent.SetSimulatePhysics` (`self.RightDoor`) true)
          (`KismetSystemLibrary.Delay` 1.0)
          (goto _label :!via `Reset`))))))

(fn `UserConstructionScript`)