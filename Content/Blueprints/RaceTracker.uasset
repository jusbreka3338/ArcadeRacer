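; RaceTracker is a race manager that lays trigger actors along a road spline.
; On BeginPlay, SpawnTriggers spawns a SplineTrigger at the world position of every RoadSpline point, ignoring collisions, and sets itself as each trigger's RaceManager.
; VehicleTrigger, presumably called back by those triggers, only prints a debug message, so no race progress is tracked here yet.
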(event `self.ReceiveBeginPlay`
  (`self.SpawnTriggers`))

(fn `SpawnTriggers`
  (for _index (range (`SplineComponent.GetNumberOfSplinePoints` (`self.RoadSpline`)))
    (bind (_returnvalue_inputkey _returnvalue_position) (break `SplinePoint` (`SplineComponent.GetSplinePointAt` (`self.RoadSpline`) _index "World")))
    (bind _returnvalue (`|SpawnActorFromClass` "/Game/Blueprints/SplineTrigger.SplineTrigger_C" (`KismetMathLibrary.MakeTransform` _returnvalue_position) "AlwaysSpawn" "MultiplyWithRoot" null null))
    (set `/Game/Blueprints/SplineTrigger.RaceManager` self _returnvalue)))

(fn `UserConstructionScript`)

(fn `VehicleTrigger`
  (`KismetSystemLibrary.PrintString` "Vehicle Triggered"))