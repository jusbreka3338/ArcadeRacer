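; ConnectPlayer_GM, apparently a game mode by its name, outlines player spawning and despawning on connect and disconnect, but is currently inert.
; Its BeginPlay, SpawnCharacter and DespawnPlayer events are empty.
; Disconnected node chains would gather PlayerStarts, destroy controlled pawns, or spawn and possess a new pawn while switching the view to GameCamera.
; None of that logic runs.
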(event `self.ReceiveBeginPlay`)

(event `SpawnCharacter`
  (params (PlayerController :type "PlayerController Object Reference")))

(event `DespawnPlayer`
  (params (PlayerController :type "PlayerController Object Reference")))

(fn `UserConstructionScript`)