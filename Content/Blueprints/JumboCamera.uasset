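; JumboCamera is a camera actor that periodically snaps to a player pawn, apparently for a large-screen view.
; Tick runs through a ten-second Delay, so SwitchCamera fires about every ten seconds with a randomly chosen camera number.
; Its only case attaches the actor to a pawn and sets a fixed offset and angle.
; Both random ranges hold a single value, so it always picks that shot and the first player index.
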(event `self.ReceiveTick`
  (params (DeltaSeconds :type "Float (single-precision)"))
  (`KismetSystemLibrary.Delay` 10.0)
  (`self.Switch Camera` (`KismetMathLibrary.RandomIntegerInRange` 1 1)))

(event `Switch Camera`
  (params (`Camera Number` :type Integer))
  (bind _returnvalue (`GameplayStatics.GetPlayerPawn` (`KismetMathLibrary.RandomIntegerInRange` 0)))
  (switch `int` `Camera Number`
    (:`1`
      (`self.K2_AttachToActor` _returnvalue "None" "KeepRelative" "KeepRelative" "KeepRelative")
      (`self.K2_SetActorLocationAndRotation` (+ (`self.K2_GetActorLocation` _returnvalue) (200.0 200.0 268.0)) (struct :`Pitch` -20.0 :`Yaw` -130.0)))))

(fn `UserConstructionScript`)