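; BP_TestWall is a test wall that drives a material bounce effect when a BP_BaseVehicle overlaps its static mesh.
; BeginPlay creates a dynamic material instance, and each vehicle overlap restarts the Bounce timeline, which writes its scaled value to the "impact" vector parameter.
; Debug prints remain, and an unconnected branch that would set a "pos" parameter from the sweep impact point never runs.
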(event `self.ReceiveBeginPlay`
  (bind _returnvalue (`PrimitiveComponent.CreateDynamicMaterialInstance` (`self.StaticMesh`) 0 null "None"))
  (set `self.Material` _returnvalue))

(event `self.StaticMesh.OnComponentBeginOverlap`
  (params (OverlappedComponent :type "PrimitiveComponent Object Reference") (OtherActor :type "Actor Object Reference") (OtherComp :type "PrimitiveComponent Object Reference") (OtherBodyIndex :type Integer) (bFromSweep :type Boolean) (SweepResult :type "HitResult Structure (by ref)"))
  (`KismetSystemLibrary.PrintString` "Hello")
  (cast `/Game/Blueprints/BP_BaseVehicle` OtherActor)
  (bind (_direction _newtrack_0) (`Timeline|bounce` :!via `PlayFromStart`)
    (:`Update`
      (bind _returnvalue (* (1.0 1.0 1.0) (* _newtrack_0 100.0)))
      (`KismetSystemLibrary.PrintString` (`KismetStringLibrary.Conv_VectorToString` _returnvalue))
      (`MaterialInstanceDynamic.SetVectorParameterValue` (`self.Material`) "impact" (`KismetMathLibrary.Conv_VectorToLinearColor` _returnvalue)))))

(fn `UserConstructionScript`)